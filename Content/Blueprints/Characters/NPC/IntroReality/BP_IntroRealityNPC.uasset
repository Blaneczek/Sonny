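; NPC for the intro reality sequence that walks along a spline path, turns and then works at a device.
; StartMoving opens a Tick-driven gate that advances the actor along the Path spline by speed while a walk animation loops.
; Near the last spline point the gate closes and a timeline turns the NPC 90 degrees.
; It then switches back to its animation Blueprint and replays a working montage every five seconds.
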(event `/Game/Blueprints/Characters/NPC/IntroReality/BPI_IntroRealityNPC.StartMoving`
  (bind _spline (`/Game/Blueprints/Characters/NPC/IntroReality/BP_IntroRealityPath.Spline` (`self.Path`)))
  (`self.Path`
    (:`then`
      (`SkeletalMeshComponent.PlayAnimation` (`self.Mesh`) "/Game/Characters/Mannequins/Animations/Manny/MM_Walk_Fwd.MM_Walk_Fwd" true)
      (goto _label :!via `Open`))
    (:`else`)))

(event `self.ReceiveTick`
  (params (DeltaSeconds :type "Float (single-precision)"))
  (bind _spline (`/Game/Blueprints/Characters/NPC/IntroReality/BP_IntroRealityPath.Spline` (`self.Path`)))
  (`/Engine/EditorBlueprintResources/StandardMacros.Gate` true :!label _label
    (:`Exit`
      (bind _output_get (set `self.Distance` (+ (`self.Distance`) (* DeltaSeconds (`self.Speed`)))))
      (bind (_returnvalue_location _returnvalue_rotation) (`KismetMathLibrary.BreakTransform` (`SplineComponent.GetTransformAtDistanceAlongSpline` (`/Game/Blueprints/Characters/NPC/IntroReality/BP_IntroRealityPath.Spline` (`self.Path`)) _output_get "World" false)))
      (`self.K2_SetActorTransform` (`KismetMathLibrary.MakeTransform` _returnvalue_location _returnvalue_rotation))
      (if (`KismetMathLibrary.NearlyEqual_FloatFloat` (`self.Distance`) (`SplineComponent.GetDistanceAlongSplineAtSplinePoint` _spline (- (`SplineComponent.GetNumberOfSplinePoints` _spline) 1)) 10.0)
        (`self.CloseGate`)
        (`self.RotateNPC`)))))

(event `CloseGate`
  (goto _label :!via `Close`))

(event `RotateNPC`
  (`SkeletalMeshComponent.PlayAnimation` (`self.Mesh`) "/Game/Characters/Mannequins/Animations/Manny/MM_Walk_InPlace.MM_Walk_InPlace" true)
  (set `self.StartRotation` (`self.K2_GetActorRotation`))
  (bind (_direction _alpha) (`Timeline|Timeline` :!via `PlayFromStart`)
    (:`Update`
      (`self.K2_SetActorRelativeRotation` (`KismetMathLibrary.RLerp` (`self.StartRotation`) (`KismetMathLibrary.ComposeRotators` (`self.StartRotation`) (struct :`Yaw` 90.0)) _alpha)))
    (:`Finished`
      (`SkeletalMeshComponent.SetAnimationMode` (`self.Mesh`) "AnimationBlueprint" true)
      (`|PlayMontage` (`self.Mesh`) "/Game/Assets/Characters/Sonny/WorkingOnDevice1_UE_Montage.WorkingOnDevice1_UE_Montage" :!label _label_2
        (:`then`
          (`KismetSystemLibrary.Delay` 5.0)
          (`self.CustomEvent`))))))

(event `CustomEvent`
  (goto _label_2))

(fn `UserConstructionScript`)