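; Supervisor NPC for the intro "line gameplay" that patrols between two tagged spawn points and catches the player (Sonny).
; A looping timer randomly halts it to turn 90 degrees and notify the player character of a check, then resumes patrol after a brief probability cooldown.
; Externally triggered seen events drive a widget bar.
; A full bar shows a death screen, then resets the supervisor and sequence.
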(event `StartLineGameplay`
  (bind _returnvalue (`KismetSystemLibrary.K2_SetTimerDelegate` (delegate `LookAroundCheck`) 2.0 true false 2.0))
  (set `self.CheckTimer` _returnvalue))

(event `SonnyCaught`
  (`KismetSystemLibrary.PrintString` "CAUGHT")
  (`self.StopLineGameplay`))

(event `LookAroundCheck`
  (bind (_returnvalue_roll _returnvalue_pitch _returnvalue_yaw) (`KismetMathLibrary.BreakRotator` (`self.K2_GetActorRotation`)))
  (`KismetSystemLibrary.PrintString` "check" true true (struct :`G` 0.66 :`B` 1.0 :`A` 1.0) 1.0)
  (if (< (`KismetMathLibrary.RandomIntegerInRange` 1 100) (`self.CheckProbability`))
    (`KismetSystemLibrary.K2_PauseTimerHandle` (`self.CheckTimer`))
    (`NavMovementInterface.StopActiveMovement` (`self.CharacterMovement`))
    (set `self.TempZRotator` _returnvalue_yaw)
    (bind (_direction _time) (`Timeline|Rotate` :!via `PlayFromStart`)
      (:`Update`
        (`self.K2_SetActorRotation` (`KismetMathLibrary.MakeRotator` 0.0 0.0 (`KismetMathLibrary.Lerp` (`self.TempZRotator`) (+ (`KismetMathLibrary.Conv_IntToDouble` (* (`self.Direction`) 90)) (`self.TempZRotator`)) _time))))
      (:`Finished`
        (`KismetSystemLibrary.PrintString` "stop check" true true (struct :`G` 0.66 :`B` 1.0 :`A` 1.0) 1.0)
        (message `/Game/Blueprints/Characters/NPC/IntroReality/BPI_IntroRealityNPC.StartSupervisorCheck` (`GameplayStatics.GetPlayerCharacter` 0) self)
        (`self.DelayGuard`)))))

(event `self.ReceiveBeginPlay`
  (set `self.tempProbability` (`self.CheckProbability`))
  (bind _aswbp_supervisor_check (cast `/Game/Blueprints/UI/Intro/WBP_SupervisorCheck` (`WidgetComponent.GetWidget` (`self.Widget`))))
  (bind _output_get (set `self.As WBP Supervisor Check` _aswbp_supervisor_check))
  (add `/Game/Blueprints/UI/Intro/WBP_SupervisorCheck.OnBarFilled` _output_get (delegate `SonnyCaught`))
  (bind _outactors (`GameplayStatics.GetAllActorsOfClassWithTag` "/Game/Blueprints/Characters/Sonny/IntroReality/BP_SpawnPoint.BP_SpawnPoint_C" "supervisor1"))
  (set `self.StartPosition` (`|GetArrayItem` _outactors))
  (bind _outactors_2 (`GameplayStatics.GetAllActorsOfClassWithTag` "/Game/Blueprints/Characters/Sonny/IntroReality/BP_SpawnPoint.BP_SpawnPoint_C" "supervisor2"))
  (set `self.EndPosition` (`|GetArrayItem` _outactors_2))
  (`KismetSystemLibrary.Delay` 20.0)
  (`self.GoToStartingPosition`)
  (`KismetSystemLibrary.Delay` 5.0)
  (`self.StartLineGameplay`))

(event `DelayGuard`
  (bind _returnvalue (`KismetSystemLibrary.K2_SetTimerDelegate` (delegate `BackToGuard`) 3.0))
  (set `self.BackToGuardTimer` _returnvalue))

(event `BackToGuard`
  (bind (_returnvalue_roll _returnvalue_pitch _returnvalue_yaw) (`KismetMathLibrary.BreakRotator` (`self.K2_GetActorRotation`)))
  (message `/Game/Blueprints/Characters/NPC/IntroReality/BPI_IntroRealityNPC.EndSupervisorCheck` (`GameplayStatics.GetPlayerCharacter` 0) self)
  (`/Game/Blueprints/UI/Intro/WBP_SupervisorCheck.ResetBar` (`self.As WBP Supervisor Check`))
  (set `self.TempZRotator` _returnvalue_yaw)
  (bind (_direction _time) (`Timeline|RotateBack` :!via `PlayFromStart`)
    (:`Update`
      (`self.K2_SetActorRotation` (`KismetMathLibrary.MakeRotator` 0.0 0.0 (`KismetMathLibrary.Lerp` (`self.TempZRotator`) (- (`self.TempZRotator`) (`KismetMathLibrary.Conv_IntToDouble` (* (`self.Direction`) 90))) _time))))
    (:`Finished`
      (if (== (`self.Direction`) 1)
        (`self.GoToStartingPosition`)
        (else
          (`self.GoToEndPosition`)))
      (set `self.CheckProbability` 0)
      (bind _returnvalue (`KismetSystemLibrary.K2_SetTimerDelegate` (delegate `BackToNormalProbability`) 4.0))
      (set `self.NormalProbabilityTimer` _returnvalue)
      (`KismetSystemLibrary.K2_UnPauseTimerHandle` (`self.CheckTimer`)))))

(event `GoToStartingPosition`
  (bind _startposition (`self.StartPosition`)
    (:`then`
      (set `self.Direction` 1)
      (bind _movementresult (`|AIMoveTo` self (0.0 0.0 0.0) _startposition)
        (:`OnSuccess`
          (`KismetSystemLibrary.PrintString` (`|GetEnumeratorNameAsString` _movementresult))
          (`KismetSystemLibrary.PrintString` "->start")
          (set `self.CheckProbability` 0)
          (`KismetSystemLibrary.Delay` 1.0)
          (set `self.CheckProbability` (`self.tempProbability`))
          (`self.GoToEndPosition`))))
    (:`else`)))

(event `BackToNormalProbability`
  (set `self.CheckProbability` (`self.tempProbability`))
  (`KismetSystemLibrary.PrintString` "back to normal" true true (struct :`G` 0.66 :`B` 1.0 :`A` 1.0) 1.0))

(event `GoToEndPosition`
  (bind _endposition (`self.EndPosition`)
    (:`then`
      (set `self.Direction` -1)
      (bind _movementresult (`|AIMoveTo` self (0.0 0.0 0.0) _endposition)
        (:`OnSuccess`
          (`KismetSystemLibrary.PrintString` (`|GetEnumeratorNameAsString` _movementresult))
          (`KismetSystemLibrary.PrintString` "->end")
          (set `self.CheckProbability` 0)
          (`KismetSystemLibrary.Delay` 1.0)
          (set `self.CheckProbability` (`self.tempProbability`))
          (`self.GoToStartingPosition`))))
    (:`else`)))

(event `/Game/Blueprints/Characters/NPC/IntroReality/BPI_IntroRealityNPC.StartSeenBySupervisor`
  (`KismetSystemLibrary.K2_ClearAndInvalidateTimerHandle` (`self.BackToGuardTimer`))
  (`KismetSystemLibrary.K2_ClearAndInvalidateTimerHandle` (`self.NormalProbabilityTimer`))
  (bind _as_wbp_supervisor_check (`self.As WBP Supervisor Check`)
    (:`then`
      (`/Game/Blueprints/UI/Intro/WBP_SupervisorCheck.StartBar` _as_wbp_supervisor_check 2.0)
      (`SceneComponent.SetVisibility` (`self.Widget`) true false))
    (:`else`)))

(event `/Game/Blueprints/Characters/NPC/IntroReality/BPI_IntroRealityNPC.EndSeenBySupervisor`
  (bind _as_wbp_supervisor_check (`self.As WBP Supervisor Check`)
    (:`then`
      (`/Game/Blueprints/UI/Intro/WBP_SupervisorCheck.StopBar` _as_wbp_supervisor_check))
    (:`else`
      _))
  (`SceneComponent.SetVisibility` (`self.Widget`) false false)
  (if (not (`KismetSystemLibrary.K2_IsTimerActiveHandle` (`self.BackToGuardTimer`)))
    (`self.DelayGuard`)))

(event `/Game/Blueprints/Characters/NPC/IntroReality/BPI_IntroRealityNPC.FinishLineGameplay`
  (bind _as_wbp_supervisor_check (`self.As WBP Supervisor Check`))
  (`/Game/Blueprints/UI/Intro/WBP_SupervisorCheck.StopBar` _as_wbp_supervisor_check)
  (`/Game/Blueprints/UI/Intro/WBP_SupervisorCheck.ResetBar` _as_wbp_supervisor_check)
  (`SceneComponent.SetVisibility` (`self.Widget`) false false)
  (`KismetSystemLibrary.K2_ClearAndInvalidateTimerHandle` (`self.CheckTimer`))
  (`KismetSystemLibrary.K2_ClearAndInvalidateTimerHandle` (`self.BackToGuardTimer`))
  (`KismetSystemLibrary.K2_ClearAndInvalidateTimerHandle` (`self.NormalProbabilityTimer`)))

(event `/Game/Blueprints/Characters/NPC/IntroReality/BPI_IntroRealityNPC.StopLineGameplay`
  (bind _as_wbp_supervisor_check (`self.As WBP Supervisor Check`))
  (message `/Game/Blueprints/Characters/NPC/IntroReality/BPI_IntroRealityNPC.StopLineGameplay` (`GameplayStatics.GetPlayerCharacter` 0))
  (`KismetSystemLibrary.K2_ClearAndInvalidateTimerHandle` (`self.CheckTimer`))
  (`KismetSystemLibrary.K2_ClearAndInvalidateTimerHandle` (`self.BackToGuardTimer`))
  (`KismetSystemLibrary.K2_ClearAndInvalidateTimerHandle` (`self.NormalProbabilityTimer`))
  (set `self.Direction` 1)
  (set `self.CheckProbability` (`self.tempProbability`))
  (`/Game/Blueprints/UI/Intro/WBP_SupervisorCheck.StopBar` _as_wbp_supervisor_check)
  (`/Game/Blueprints/UI/Intro/WBP_SupervisorCheck.ResetBar` _as_wbp_supervisor_check)
  (`SceneComponent.SetVisibility` (`self.Widget`) false false)
  (bind _returnvalue (`|CreateWidget` "/Game/Blueprints/UI/Intro/WBP_LineDeathScreen.WBP_LineDeathScreen_C"))
  (`UserWidget.AddToViewport` _returnvalue 0)
  (`KismetSystemLibrary.Delay` 3.0)
  (`self.ResetLineGameplay`))

(event `/Game/Blueprints/Characters/NPC/IntroReality/BPI_IntroRealityNPC.ResetLineGameplay`
  (message `/Game/Blueprints/Characters/NPC/IntroReality/BPI_IntroRealityNPC.ResetLineGameplay` (`GameplayStatics.GetPlayerCharacter` 0))
  (`self.K2_SetActorTransform` (`self.GetTransform` (`self.StartPosition`)))
  (`KismetSystemLibrary.Delay` 2.0)
  (`self.StartLineGameplay`)
  (`self.GoToEndPosition`))

(fn `UserConstructionScript`)