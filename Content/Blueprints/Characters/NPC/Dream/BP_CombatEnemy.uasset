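; Enemy character for the sectioned combat mode: it hears the player, breaks blocks and ends combat on contact.
; Combat, section, slow-down and reset events drive the AI controller's state and walk speed, which is reduced by a game mode stat.
; Hearing sphere changes state for a same-section player; attack sphere updates score, stops all combat actors and resets blockers.
; A montage notify triggers block interaction, and first deactivation grants the player blocks.
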(event `/Game/Blueprints/Systems/Combat/BPI_Combat.StartCombat`
  (params (ForwardVector :type "Vector Structure") (ResetLocation :type "Vector Structure") (Level :type "/Game/Blueprints/Systems/E_GameplayLevel Enum" :default "NewEnumerator3"))
  (`KismetSystemLibrary.Delay` 1.0)
  (`self.SetStats`)
  (set `self.StartingLocation` (`self.K2_GetActorLocation`))
  (`self.SetSpeed` "NewEnumerator0")
  (`self.SectionChange` 0))

(event `SetDeactivatedState`
  (params (IsDeactivated :type Boolean))
  (bind _output_get (set `self.bDeactivated` IsDeactivated))
  (if (and _output_get (not (`self.bWasDeactivatedBefore`)))
    (set `self.bWasDeactivatedBefore` true)
    (message `/Game/Blueprints/Systems/Combat/BPI_Combat.AddBlocks` (`GameplayStatics.GetPlayerCharacter` 0) 4)))

(event `self.SphereAttack.OnComponentBeginOverlap`
  (params (OverlappedComponent :type "PrimitiveComponent Object Reference") (OtherActor :type "Actor Object Reference") (OtherComp :type "PrimitiveComponent Object Reference") (OtherBodyIndex :type Integer) (bFromSweep :type Boolean) (SweepResult :type "HitResult Structure (by ref)"))
  (if (`self.bIsCurrentSectionActive`)
    (if (== OtherActor (`GameplayStatics.GetPlayerCharacter` 0))
      (message `/Game/Blueprints/GameModes/Dreams/BPI_DreamGameMode.UpdateCombatModeScore` (`GameplayStatics.GetGameMode`) "NewEnumerator4")
      (bind _outactors (`GameplayStatics.GetAllActorsWithInterface` "/Game/Blueprints/Systems/Combat/BPI_Combat.BPI_Combat_C"))
      (for _array_element _outactors
        (message `/Game/Blueprints/Systems/Combat/BPI_Combat.StopCombat` _array_element))
      (bind _outactors_2 (`GameplayStatics.GetAllActorsOfClass` "/Game/Blueprints/Systems/BP_Blocker.BP_Blocker_C"))
      (for _array_element_2 _outactors_2
        (`/Engine/EditorBlueprintResources/StandardMacros.IsValid` _array_element_2
          (:`Is Valid`
            (`/Game/Blueprints/Systems/BP_Blocker.ResetCollision` _array_element_2)))))))

(event `self.SphereHearing.OnComponentBeginOverlap`
  (params (OverlappedComponent :type "PrimitiveComponent Object Reference") (OtherActor :type "Actor Object Reference") (OtherComp :type "PrimitiveComponent Object Reference") (OtherBodyIndex :type Integer) (bFromSweep :type Boolean) (SweepResult :type "HitResult Structure (by ref)"))
  (bind _state (message `/Game/Blueprints/Systems/Combat/AI/BPI_EnemyAI.GetState` (`self.GetController`)))
  (if (and (`self.bIsCurrentSectionActive`) (`|EnumEquality` _state "NewEnumerator0"))
    (if (== OtherActor (`GameplayStatics.GetPlayerCharacter` 0))
      (bind _sectionindex (message `/Game/Blueprints/Systems/Combat/BPI_Combat.GetSectionIndex` OtherActor))
      (if (== (`self.SectionIndex`) _sectionindex)
        (message `/Game/Blueprints/Systems/Combat/AI/BPI_EnemyAI.SetState` (`self.GetController`) "NewEnumerator1")))))

(event `/Game/Blueprints/Systems/Combat/BPI_Combat.BlockDestroyed`
  (message `/Game/Blueprints/Systems/Combat/AI/BPI_EnemyAI.SetState` (`self.GetController`) "NewEnumerator1"))

(event `/Game/Blueprints/Systems/Combat/BPI_Combat.DestroyBlock`
  (params (BlockActor :type "Actor Object Reference"))
  (`/Engine/EditorBlueprintResources/StandardMacros.IsValid` BlockActor
    (:`Is Valid`
      (bind _notifyname (`|PlayMontage` (`self.Mesh`) "/Game/Assets/Characters/ZombieRobot/Enemy_Attack1_Montage.Enemy_Attack1_Montage" 0.7)
        (:`OnCompleted`
          (`self.OnEndHit` :!label _label))
        (:`OnInterrupted`
          (goto _label))
        (:`OnNotifyBegin`
          (switch `name` _notifyname
            (:`Attack`
              (`/Engine/EditorBlueprintResources/StandardMacros.IsValid` BlockActor
                (:`Is Valid`
                  (message `/Game/Blueprints/Systems/Interaction/BPI_Interaction.OnInteract` BlockActor self))))))))))

(event `/Game/Blueprints/Systems/Combat/BPI_Combat.StopCombat`
  (message `/Game/Blueprints/Systems/Combat/AI/BPI_EnemyAI.SetState` (`self.GetController`) "NewEnumerator4"))

(event `/Game/Blueprints/Systems/Combat/BPI_Combat.ResetCombat`
  (set `self.bSlowed` false)
  (set `self.bWasDeactivatedBefore` false)
  (set `self.bDeactivated` false)
  (`self.K2_SetActorLocation` (`self.StartingLocation`))
  (`KismetSystemLibrary.Delay` 1.0)
  (message `/Game/Blueprints/Systems/Combat/AI/BPI_EnemyAI.SetState` (`self.GetController`) "NewEnumerator0"))

(event `/Game/Blueprints/Systems/Combat/BPI_Combat.SectionChange`
  (params (SectionIndex :type Integer))
  (if (== SectionIndex (`self.SectionIndex`))
    (set `self.bIsCurrentSectionActive` true)
    (message `/Game/Blueprints/Systems/Combat/AI/BPI_EnemyAI.SetState` (`self.GetController`) "NewEnumerator0")
    (else
      (set `self.bIsCurrentSectionActive` false)
      (message `/Game/Blueprints/Systems/Combat/AI/BPI_EnemyAI.SetState` (`self.GetController`) "NewEnumerator4"))))

(event `/Game/Blueprints/Systems/Combat/BPI_Combat.SlowDown`
  (params (IsSlowed :type Boolean))
  (bind _state (message `/Game/Blueprints/Systems/Combat/AI/BPI_EnemyAI.GetState` (`self.GetController`)))
  (if (`|EnumEquality` _state "NewEnumerator1")
    (if IsSlowed
      (set `CharacterMovementComponent.MaxWalkSpeed` (/ (`self.StarterCombatWalkSpeed`) 2.0) (`self.CharacterMovement`))
      (set `self.bSlowed` true)
      (else
        (set `CharacterMovementComponent.MaxWalkSpeed` (`self.StarterCombatWalkSpeed`) (`self.CharacterMovement`))
        (set `self.bSlowed` false)))
    (elif (`self.bSlowed`)
      (set `CharacterMovementComponent.MaxWalkSpeed` (`self.StarterCombatWalkSpeed`) (`self.CharacterMovement`))
      (set `self.bSlowed` false))))

(fn `GetAttackDamageValue`
  (returns (Value :type "Float (double-precision)"))
  (return (`self.AttackDamage`)))

(fn `GetNumberOfSlowdownUses`
  (returns (Uses :type Integer))
  (return 0))

(fn `GetSectionIndex`
  (returns (SectionIndex :type Integer))
  (return 0))

(fn `SetSpeed`
  (params (NewSpeed :type "/Game/Blueprints/Systems/Combat/AI/E_EnemySpeed Enum" :default "NewEnumerator0"))
  (switch `/Game/Blueprints/Systems/Combat/AI/E_EnemySpeed` NewSpeed
    (:`NewEnumerator0`
      (set `CharacterMovementComponent.MaxWalkSpeed` 80.0 (`self.CharacterMovement`)))
    (:`NewEnumerator1`
      (set `CharacterMovementComponent.MaxWalkSpeed` (`self.StarterCombatWalkSpeed`) (`self.CharacterMovement`)))))

(fn `SetStats`
  (bind _stats (message `/Game/Blueprints/GameModes/Dreams/BPI_DreamGameMode.GetCombatStats` (`GameplayStatics.GetGameMode`)))
  (set `self.StarterCombatWalkSpeed` (- 350.0 (`BlueprintMapLibrary.Map_Find` _stats "NewEnumerator1"))))

(fn `UserConstructionScript`)