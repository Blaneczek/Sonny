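; Dialogue NPC that starts its conversation automatically the first time the player enters its sphere, then enables an interaction prompt.
; Interaction turns NPC and player to face each other through a timeline-driven yaw interpolation and starts the dialogue component, passing the first-time flag.
; BeginPlay restores that flag by NameTag from GameInstance data and delays enabling sphere collision.
; Dialogue end clears the flag and requests a save through the GameMode.
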(event `self.ReceiveBeginPlay`
  (`self.LoadSaveData`)
  (`KismetSystemLibrary.Delay` 1.0)
  (`PrimitiveComponent.SetCollisionEnabled` (`self.Sphere`) "QueryOnly"))

(event `Stop`
  (bind _returnvalue (`GameplayStatics.GetPlayerCharacter` 0))
  (bind (_returnvalue_roll _returnvalue_pitch _returnvalue_yaw) (`KismetMathLibrary.BreakRotator` (`KismetMathLibrary.RInterpTo` (`self.K2_GetActorRotation`) (`self.TargetRotation`) (`GameplayStatics.GetWorldDeltaSeconds`) 2.0)))
  (bind (_returnvalue_roll_2 _returnvalue_pitch_2 _returnvalue_yaw_2) (`KismetMathLibrary.BreakRotator` (`KismetMathLibrary.RInterpTo` (`self.K2_GetActorRotation` _returnvalue) (`self.TargetRotation2`) (`GameplayStatics.GetWorldDeltaSeconds`) 2.0)))
  (`Timeline|Rotate` :!via `Stop` :!label _label
    (:`Update`
      (`self.K2_SetActorRotation` (`KismetMathLibrary.MakeRotator` 0.0 0.0 _returnvalue_yaw))
      (`self.K2_SetActorRotation` _returnvalue (`KismetMathLibrary.MakeRotator` 0.0 0.0 _returnvalue_yaw_2) false))))

(event `RotateToPlayer`
  (set `self.TargetRotation` (`KismetMathLibrary.FindLookAtRotation` (`self.K2_GetActorLocation`) (`self.K2_GetActorLocation` (`GameplayStatics.GetPlayerCharacter` 0))))
  (set `self.TargetRotation2` (`KismetMathLibrary.FindLookAtRotation` (`self.K2_GetActorLocation` (`GameplayStatics.GetPlayerCharacter` 0)) (`self.K2_GetActorLocation`)))
  (goto _label :!via `PlayFromStart`))

(event `/Game/Blueprints/Systems/Interaction/BPI_Interaction.ShowPrompt`
  (if (`self.bCanShowPrompt`)
    (`/Game/Blueprints/Systems/Interaction/BPC_Interaction.ShowPrompt` (`self.BPC_Interaction`))))

(event `/Game/Blueprints/Systems/Interaction/BPI_Interaction.HidePromt`
  (`/Game/Blueprints/Systems/Interaction/BPC_Interaction.HidePrompt` (`self.BPC_Interaction`)))

(event `/Game/Blueprints/Systems/Interaction/BPI_Interaction.OnInteract`
  (params (Actor :type "Actor Object Reference"))
  (`/Game/Blueprints/Systems/Interaction/BPC_Interaction.Interact` (`self.BPC_Interaction`) true))

(event `self.BPC_Interaction.OnInteract`
  (params (CanInteract :type Boolean))
  (if CanInteract
    (`self.RotateToPlayer`)
    (`/Game/Blueprints/Systems/Dialogues/BPC_Dialogue.StartDialog` (`self.BPC_Dialogue`) (`self.bFirstTimeDialogue`))))

(event `self.Sphere.OnComponentBeginOverlap`
  (params (OverlappedComponent :type "PrimitiveComponent Object Reference") (OtherActor :type "Actor Object Reference") (OtherComp :type "PrimitiveComponent Object Reference") (OtherBodyIndex :type Integer) (bFromSweep :type Boolean) (SweepResult :type "HitResult Structure (by ref)"))
  (if (and (== OtherActor (`GameplayStatics.GetPlayerCharacter` 0)) (`self.bFirstTimeDialogue`))
    (`KismetSystemLibrary.PrintString` "ssssssss")
    (`/Engine/EditorBlueprintResources/StandardMacros.DoOnce` false
      (:`Completed`
        (set `self.bCanShowPrompt` true)
        (set `/Game/Blueprints/Systems/Interaction/BPC_Interaction.CanInteract` true (`self.BPC_Interaction`))
        (`self.OnInteract` null)))))

(event `self.BPC_Dialogue.OnDialogueEnd`
  (set `self.bFirstTimeDialogue` false)
  (message `/Game/Blueprints/GameModes/Dreams/BPI_DreamGameMode.SaveGame` (`GameplayStatics.GetGameMode`)))

(fn `LoadSaveData`
  (bind _savegamedata (message `/Game/Blueprints/Systems/Saves/BPI_SaveGame.GetGameData` (`GameplayStatics.GetGameInstance`)))
  (bind (_value _returnvalue) (`BlueprintMapLibrary.Map_Find` (`.DialogueNPC_18_09A48BA943DC5C846796748062E21DF8` (break `/Game/Blueprints/Systems/Saves/S_SaveData` _savegamedata)) (`self.NameTag`)))
  (if _returnvalue
    (bind _output_get (set `self.bFirstTimeDialogue` _value))
    (set `self.bCanShowPrompt` (not _output_get))))

(fn `UserConstructionScript`)