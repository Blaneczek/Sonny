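; Dream NPC flying wolf that wanders on foot until triggered to fly away along a spline path.
; While idle it loops AI moves to random nearby navigable points with a short pause.
; FlyYouFool clears its tags and walks it to the given path actor's spline start, resuming wandering if that move fails.
; A gated Tick then moves it collision-free along the spline and destroys it at the end.
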(event `self.ReceiveBeginPlay`
  (`self.FreeWalk`))

(event `FreeWalk`
  (if (not (`self.bFlying`))
    (bind _randomlocation (`NavigationSystemV1.K2_GetRandomLocationInNavigableRadius` (`self.K2_GetActorLocation`) 600.0 null null))
    (bind _output_get (set `self.Random Location` _randomlocation))
    (`|AIMoveTo` self _output_get null
      (:`OnSuccess`
        _)
      (:`OnFail`
        _))
    (`KismetSystemLibrary.Delay` 1.0)
    (`self.FreeWalk`)))

(event `FlyYouFool`
  (params (PathActor :type "/Game/Blueprints/Systems/Narrative/BP_FlyingWolfPath Object Reference") (NewTag :type Name))
  (bind _spline (`/Game/Blueprints/Systems/Narrative/BP_FlyingWolfPath.Spline` PathActor))
  (`KismetArrayLibrary.Array_Clear` (`self.Tags`))
  (set `self.bFlying` true)
  (`MovementComponent.StopMovementImmediately` (`self.CharacterMovement`))
  (`/Engine/EditorBlueprintResources/StandardMacros.IsValid` PathActor
    (:`Is Valid`
      (set `self.Spline` _spline)
      (`|AIMoveTo` self (`SplineComponent.GetLocationAtSplinePoint` _spline 0 "World") null 10.0
        (:`OnSuccess`
          (set `self.bJump` true)
          (`self.Fly`)
          (`self.SetActorEnableCollision` false))
        (:`OnFail`
          (set `self.bFlying` false)
          (`self.FreeWalk`))))))

(event `Fly`
  (bind _spline (`self.Spline`))
  (set `self.Distance` 0.0)
  (goto _label :!via `Open`))

(event `self.ReceiveTick`
  (params (DeltaSeconds :type "Float (single-precision)"))
  (bind _spline (`self.Spline`))
  (`/Engine/EditorBlueprintResources/StandardMacros.Gate` true :!label _label
    (:`Exit`
      (bind _output_get (set `self.Distance` (+ (* DeltaSeconds (`self.FlyingSpeed`)) (`self.Distance`))))
      (`self.K2_SetActorLocation` (`SplineComponent.GetLocationAtDistanceAlongSpline` _spline _output_get "World"))
      (`self.K2_SetActorRotation` (`SplineComponent.GetRotationAtDistanceAlongSpline` _spline _output_get "World"))
      (if (>= (`self.Distance`) (`SplineComponent.GetSplineLength` (`self.Spline`)))
        (`self.K2_DestroyActor`)))))

(event `CloseTick`
  (goto _label :!via `Close`))

(fn `UserConstructionScript`)