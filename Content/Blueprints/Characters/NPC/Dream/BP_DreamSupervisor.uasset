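; Dream NPC supervisor for line mode that patrols randomly and catches the player with a colored vision cone.
; It turns toward a random reachable point via Timeline, moves there with AIMoveTo, and sometimes changes course on a looping timer.
; Setup reduces starter speed and cone size using game mode stats.
; Catching the player updates score, resets line blocks and interface-stops line mode actors; the supervisor then returns to start and resumes.
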(event `self.ReceiveBeginPlay`
  (`self.SaveStarterStats`)
  (set `self.StartLocation` (`self.K2_GetActorLocation`))
  (`self.SetConeColor` (`self.ColorDefault`) (`self.Opacity`)))

(event `/Game/Blueprints/Systems/LineMode/Dream/BPI_LineModeDream.LineModeSetup`
  (params (ForwardVector :type "Vector Structure") (Level :type "/Game/Blueprints/Systems/E_GameplayLevel Enum" :default "NewEnumerator3") (ResetLocation :type "Vector Structure"))
  (bind _output_get (set `self.bActive` (`|EnumEquality` Level (`self.Level`))))
  (if _output_get
    (bind _stats (message `/Game/Blueprints/GameModes/Dreams/BPI_DreamGameMode.GetLineModeStats` (`GameplayStatics.GetGameMode`)))
    (`self.SetStats` (- (`self.StarterSpeed`) (`BlueprintMapLibrary.Map_Find` _stats "NewEnumerator2")) (- (`self.StarterConeScale`) (`BlueprintMapLibrary.Map_Find` _stats "NewEnumerator3")))
    (`self.RotateToLocation`)))

(event `RotateToLocation`
  (bind _returnvalue (`KismetSystemLibrary.K2_SetTimerDelegate` (delegate `RotateDelay`) 0.5))
  (set `self.RotateDelayTimer` _returnvalue))

(event `StopRotate`
  (bind (_random_location_x _random_location_y) (`KismetMathLibrary.BreakVector` (`self.Random Location`)))
  (bind (_desiredrotation_roll _desiredrotation_pitch _desiredrotation_yaw) (`KismetMathLibrary.BreakRotator` (`self.DesiredRotation`)))
  (bind (_startlocation_x _startlocation_y _startlocation_z) (`KismetMathLibrary.BreakVector` (`self.StartLocation`)))
  (bind _yaw (.yaw (`KismetMathLibrary.RInterpTo_Constant` (`self.K2_GetActorRotation`) (`self.DesiredRotation`) (`GameplayStatics.GetWorldDeltaSeconds`) 50.0)))
  (`Timeline|Timeline` :!via `Stop` :!label _label
    (:`Update`
      (if (`KismetMathLibrary.NearlyEqual_FloatFloat` _yaw _desiredrotation_yaw 1.0)
        (`self.StopRotate`)
        (`self.MoveTo` (`KismetMathLibrary.MakeVector` _random_location_x _random_location_y (+ _startlocation_z 50.0)))
        (else
          (`self.K2_SetActorRotation` (`KismetMathLibrary.MakeRotator` 0.0 0.0 _yaw)))))))

(event `RotateDelay`
  (set `self.Random Location` (`NavigationSystemV1.K2_GetRandomReachablePointInRadius` (`self.K2_GetActorLocation`) 2000.0 null null))
  (set `self.DesiredRotation` (`KismetMathLibrary.FindLookAtRotation` (`self.K2_GetActorLocation`) (`self.Random Location`)))
  (goto _label :!via `PlayFromStart`))

(event `MoveTo`
  (params (Location :type "Vector Structure"))
  (`|AIMoveTo` self Location null 10.0
    (:`then`
      (bind _returnvalue (`KismetSystemLibrary.K2_SetTimerDelegate` (delegate `RandomPathChange`) 2.0 true))
      (set `self.RandomPathChangeTimer` _returnvalue))
    (:`OnSuccess`
      (`KismetSystemLibrary.K2_ClearAndInvalidateTimerHandle` (`self.RandomPathChangeTimer`))
      (`self.RotateToLocation`))))

(event `RandomPathChange`
  (if (<= (`KismetMathLibrary.RandomIntegerInRange` 0 100) 30)
    (`KismetSystemLibrary.K2_ClearAndInvalidateTimerHandle` (`self.RandomPathChangeTimer`))
    (`NavMovementInterface.StopActiveMovement` (`self.CharacterMovement`))
    (`self.RotateToLocation`)))

(event `self.Cone.OnComponentBeginOverlap`
  (params (OverlappedComponent :type "PrimitiveComponent Object Reference") (OtherActor :type "Actor Object Reference") (OtherComp :type "PrimitiveComponent Object Reference") (OtherBodyIndex :type Integer) (bFromSweep :type Boolean) (SweepResult :type "HitResult Structure (by ref)"))
  (if (and (== OtherActor (`GameplayStatics.GetPlayerCharacter` 0)) (not (`self.bCaughtSonny`)))
    (message `/Game/Blueprints/GameModes/Dreams/BPI_DreamGameMode.UpdateLineModeScore` (`GameplayStatics.GetGameMode`) "NewEnumerator1")
    (`self.SetConeColor` (`self.ColorCaught`) (`self.Opacity`))
    (bind _outactors (`GameplayStatics.GetAllActorsOfClass` "/Game/Blueprints/Systems/LineMode/Dream/BP_LineBlockDream.BP_LineBlockDream_C"))
    (for _array_element _outactors
      (message `/Game/Blueprints/Systems/LineMode/BPI_Lines.Reset` _array_element))
    (bind _outactors_2 (`GameplayStatics.GetAllActorsWithInterface` "/Game/Blueprints/Systems/LineMode/Dream/BPI_LineModeDream.BPI_LineModeDream_C"))
    (for _array_element_2 _outactors_2
      (message `/Game/Blueprints/Systems/LineMode/Dream/BPI_LineModeDream.StopLineMode` _array_element_2))))

(event `/Game/Blueprints/Systems/LineMode/Dream/BPI_LineModeDream.ResetLineMode`
  (if (`self.bActive`)
    (`self.SetConeColor` (`self.ColorDefault`) (`self.Opacity`))
    (`self.K2_SetActorLocation` (`self.StartLocation`))
    (`KismetSystemLibrary.Delay` 2.0)
    (`self.RotateToLocation`)
    (set `self.bCaughtSonny` false)))

(event `/Game/Blueprints/Systems/LineMode/Dream/BPI_LineModeDream.StopLineMode`
  (if (`self.bActive`)
    (set `self.bCaughtSonny` true)
    (`KismetSystemLibrary.K2_ClearAndInvalidateTimerHandle` (`self.RandomPathChangeTimer`))
    (`KismetSystemLibrary.K2_ClearAndInvalidateTimerHandle` (`self.RotateDelayTimer`))
    (`MovementComponent.StopMovementImmediately` (`self.CharacterMovement`))
    (`self.StopRotate`)
    (`KismetSystemLibrary.Delay` 2.0)
    (`self.ResetLineMode`)))

(event `/Game/Blueprints/Systems/LineMode/Dream/BPI_LineModeDream.FinishLineMode`
  (if (`self.bActive`)
    (`NavMovementInterface.StopActiveMovement` (`self.CharacterMovement`))
    (`self.StopRotate`)
    (`self.SetStats` (`self.StarterSpeed`) (`self.StarterConeScale`))))

(fn `GetInvisibilityCurrentIndex`)

(fn `GetNumberOfInvisibilityUses`
  (returns (Uses :type Integer))
  (return 0))

(fn `IsInvisible`
  (returns (Invisible :type Boolean))
  (return false))

(fn `SaveStarterStats`
  (set `self.StarterSpeed` (`CharacterMovementComponent.MaxWalkSpeed` (`self.CharacterMovement`)))
  (set `self.StarterConeScale` (.z (`SceneComponent.RelativeScale3D` (`self.Cone`)))))

(fn `SetConeColor`
  (params (Color :type "LinearColor Structure") (Opacity :type "Float (single-precision)"))
  (bind _returnvalue (`PrimitiveComponent.CreateDynamicMaterialInstance` (`self.Cone`) 0 "/Game/Assets/Materials/Dream/MI_SupervisorCone.MI_SupervisorCone" "None"))
  (`MaterialInstanceDynamic.SetVectorParameterValue` _returnvalue "Color" Color)
  (`MaterialInstanceDynamic.SetScalarParameterValue` _returnvalue "Opacity" Opacity)
  (return))

(fn `SetConeScale`
  (params (NewScale :type "Float (double-precision)"))
  (`SceneComponent.SetRelativeScale3D` (`self.Cone`) (`KismetMathLibrary.MakeVector` 0.1 NewScale NewScale))
  (`SceneComponent.K2_SetRelativeLocation` (`self.Cone`) (`KismetMathLibrary.MakeVector` (- 115.0 (* (/ (- 2.0 NewScale) 0.05) 2.5)) 0.0 15.0) false false))

(fn `SetStats`
  (params (Speed :type "Float (double-precision)") (ConeScale :type "Float (double-precision)"))
  (set `CharacterMovementComponent.MaxFlySpeed` Speed (`self.CharacterMovement`))
  (`self.SetConeScale` ConeScale))

(fn `UserConstructionScript`)