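; Player character for Sonny's dream, switching between default exploration, Line Mode path puzzles and grid-based Combat.
; Each mode sets spring-arm camera and controls, locking yaw to a given direction outside default.
; Line Mode chains overlapped BPI_Lines blocks while the mouse is held, with death-screen reset.
; Combat spawns grid-snapped blocks on clicked floors; per-tick traces from camera or actor drive interaction prompts through interfaces.
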(event `Key|LeftMouseButton`
  (params (Key :type "Key Structure"))
  (bind (_bblockinghit _binitialoverlap _time _distance _location _impactpoint _normal _impactnormal _physmat _hitactor) (`GameplayStatics.BreakHitResult` (`PlayerController.GetHitResultUnderCursorForObjects` (`GameplayStatics.GetPlayerController` 0) (`|MakeArray` "ObjectTypeQuery7" :!type "EObjectTypeQuery Enum") true)))
  ;[0.1476 0.15 0.003822 0.5] Mouse actions
  (:`Pressed`
    (switch `/Game/Blueprints/Characters/Sonny/Dream/E_GameplayType` (`self.GameplayType`)
      (:`NewEnumerator1`
        (set `self.bDrawLinePath` true)
        (`MeshComponent.SetOverlayMaterial` (`self.Mesh`) "/Game/Assets/Materials/Dream/M_SonnyGlow_Inst.M_SonnyGlow_Inst"))
      (:`NewEnumerator2`
        (if (`KismetSystemLibrary.DoesImplementInterface` _hitactor "/Game/Blueprints/Systems/Combat/BPI_CombatFloor.BPI_CombatFloor_C")
          (`self.SpawnCombatBlock` _hitactor)))))
  (:`Released`
    (switch `/Game/Blueprints/Characters/Sonny/Dream/E_GameplayType` (`self.GameplayType`)
      (:`NewEnumerator1`
        (set `self.bDrawLinePath` false)
        (`MeshComponent.SetOverlayMaterial` (`self.Mesh`) null)))))

(event `self.ReceiveBeginPlay`
  (`self.SetCameraPosition` (`self.DefaultTargetArmLength`)))

(event `self.ReceiveTick`
  (params (DeltaSeconds :type "Float (single-precision)"))
  (`self.LineTrace`))

(event `Key|E`
  (params (Key :type "Key Structure"))
  (:`Pressed`
    (switch `/Game/Blueprints/Characters/Sonny/Dream/E_GameplayType` (`self.GameplayType`)
      (:`NewEnumerator0`
        (message `/Game/Blueprints/Systems/Interaction/BPI_Interaction.OnInteract` (`self.Hit Actor`) self)))))

(event `self.CapsuleComponent.OnComponentBeginOverlap`
  (params (OverlappedComponent :type "PrimitiveComponent Object Reference") (OtherActor :type "Actor Object Reference") (OtherComp :type "PrimitiveComponent Object Reference") (OtherBodyIndex :type Integer) (bFromSweep :type Boolean) (SweepResult :type "HitResult Structure (by ref)"))
  (if (`KismetSystemLibrary.DoesImplementInterface` OtherActor "/Game/Blueprints/Systems/LineMode/BPI_Lines.BPI_Lines_C")
    (if (and (== (`self.HittedBlock`) (`self.SteppedBlock`)) (`self.bDrawLinePath`))
      (bind _available (message `/Game/Blueprints/Systems/LineMode/BPI_Lines.IsAvailable` OtherActor))
      (if _available
        (message `/Game/Blueprints/Systems/LineMode/BPI_Lines.HighlightBlock` OtherActor (`self.HittedBlock`))
        (set `self.HittedBlock` OtherActor)))))

(event `self.CapsuleComponent.OnComponentEndOverlap`
  (params (OverlappedComponent :type "PrimitiveComponent Object Reference") (OtherActor :type "Actor Object Reference") (OtherComp :type "PrimitiveComponent Object Reference") (OtherBodyIndex :type Integer))
  (if (`KismetSystemLibrary.DoesImplementInterface` OtherActor "/Game/Blueprints/Systems/LineMode/BPI_Lines.BPI_Lines_C")
    (set `self.SteppedBlock` OtherActor)))

(event `/Game/Blueprints/Systems/LineMode/Dream/BPI_LineModeDream.LineModeSetup`
  (params (ForwardVector :type "Vector Structure"))
  (bind (_returnvalue_roll _returnvalue_pitch _returnvalue_yaw) (`KismetMathLibrary.BreakRotator` (`KismetMathLibrary.Conv_VectorToRotator` ForwardVector)))
  (bind (_linemodecamerarotation_roll _linemodecamerarotation_pitch) (`KismetMathLibrary.BreakRotator` (`self.LineModeCameraRotation`)))
  ;[0.01516 0.15 0.05225 0.5] LineModeGameplay
  (set `self.GameplayType` "NewEnumerator1")
  (`self.SetCameraPosition` (`self.LineModeTargetArmLength`) (`KismetMathLibrary.MakeRotator` _linemodecamerarotation_roll _linemodecamerarotation_pitch _returnvalue_yaw))
  (`self.SetControlls` _returnvalue_yaw))

(event `/Game/Blueprints/Systems/LineMode/Dream/BPI_LineModeDream.ResetLineMode`
  ;[0.01516 0.15 0.05225 0.5] LineModeGameplay
  (set `self.bDrawLinePath` false)
  (bind _returnvalue (`GameplayStatics.GetActorOfClass` "/Game/Blueprints/Systems/LineMode/Dream/BP_LineModeStarter.BP_LineModeStarter_C"))
  (`/Engine/EditorBlueprintResources/StandardMacros.IsValid` _returnvalue
    (:`Is Valid`
      (`self.K2_SetActorLocation` (`self.K2_GetActorLocation` _returnvalue))
      (`self.EnableInput` (`GameplayStatics.GetPlayerController` 0)))))

(event `/Game/Blueprints/Systems/LineMode/Dream/BPI_LineModeDream.StopLineMode`
  ;[0.01516 0.15 0.05225 0.5] LineModeGameplay
  (`self.DisableInput` (`GameplayStatics.GetPlayerController` 0))
  (set `self.HittedBlock` null)
  (set `self.SteppedBlock` null)
  (`KismetSystemLibrary.Delay` 1.0)
  (bind _returnvalue (`|CreateWidget` "/Game/Blueprints/UI/Intro/WBP_LineDeathScreen.WBP_LineDeathScreen_C"))
  (`UserWidget.AddToViewport` _returnvalue 0)
  (`KismetSystemLibrary.Delay` 2.0)
  (`self.ResetLineMode`))

(event `/Game/Blueprints/Systems/LineMode/Dream/BPI_LineModeDream.SetFirstBlockRef`
  (params (FirstBlock :type "/Game/Blueprints/Systems/LineMode/Dream/BP_LineBlockDream Object Reference"))
  ;[0.01516 0.15 0.05225 0.5] LineModeGameplay
  (set `self.HittedBlock` FirstBlock))

(event `/Game/Blueprints/Systems/LineMode/Dream/BPI_LineModeDream.FinishLineMode`
  ;[0.01516 0.15 0.05225 0.5] LineModeGameplay
  (set `self.GameplayType` "NewEnumerator0")
  (`self.SetCameraPosition` (`self.DefaultTargetArmLength`))
  (`self.SetControlls` 0.0)
  (`MeshComponent.SetOverlayMaterial` (`self.Mesh`) null))

(event `/Game/Blueprints/Systems/Combat/BPI_Combat.StartCombat`
  (params (ForwardVector :type "Vector Structure"))
  (bind (_returnvalue_roll _returnvalue_pitch _returnvalue_yaw) (`KismetMathLibrary.BreakRotator` (`KismetMathLibrary.Conv_VectorToRotator` ForwardVector)))
  (bind (_combatcamerarotation_roll _combatcamerarotation_pitch) (`KismetMathLibrary.BreakRotator` (`self.CombatCameraRotation`)))
  (set `self.GameplayType` "NewEnumerator2")
  (`self.SetCameraPosition` (`self.CombatTargetArmLength`) (`KismetMathLibrary.MakeRotator` _combatcamerarotation_roll _combatcamerarotation_pitch _returnvalue_yaw))
  (`self.SetControlls` _returnvalue_yaw)
  (set `PlayerController.bShowMouseCursor` true (`GameplayStatics.GetPlayerController` 0)))

(event `self.SphereCombatFloorCheck.OnComponentBeginOverlap`
  (params (OverlappedComponent :type "PrimitiveComponent Object Reference") (OtherActor :type "Actor Object Reference") (OtherComp :type "PrimitiveComponent Object Reference") (OtherBodyIndex :type Integer) (bFromSweep :type Boolean) (SweepResult :type "HitResult Structure (by ref)"))
  (if (`KismetSystemLibrary.DoesImplementInterface` OtherActor "/Game/Blueprints/Systems/Combat/BPI_CombatFloor.BPI_CombatFloor_C")
    (message `/Game/Blueprints/Systems/Combat/BPI_CombatFloor.SonnyInRange` OtherActor)))

(event `self.SphereCombatFloorCheck.OnComponentEndOverlap`
  (params (OverlappedComponent :type "PrimitiveComponent Object Reference") (OtherActor :type "Actor Object Reference") (OtherComp :type "PrimitiveComponent Object Reference") (OtherBodyIndex :type Integer))
  (if (`KismetSystemLibrary.DoesImplementInterface` OtherActor "/Game/Blueprints/Systems/Combat/BPI_CombatFloor.BPI_CombatFloor_C")
    (message `/Game/Blueprints/Systems/Combat/BPI_CombatFloor.SonnyOutRange` OtherActor)))

(event `Key|SpaceBar`
  (params (Key :type "Key Structure"))
  (:`Pressed`
    (switch `/Game/Blueprints/Characters/Sonny/Dream/E_GameplayType` (`self.GameplayType`)
      (:`NewEnumerator2`
        (message `/Game/Blueprints/Systems/Interaction/BPI_Interaction.OnInteract` (`self.Hit Actor`) self)))))

(event `/Game/Blueprints/Systems/LineMode/Dream/BPI_LineModeDream.NullBlock`
  (set `self.SteppedBlock` null))

(event `/Game/Blueprints/Systems/Combat/BPI_Combat.SectionChange`
  (params (SectionIndex :type Integer))
  (set `self.CurrentSectionIndex` SectionIndex))

(fn `GetAttackDamageValue`
  (returns (Value :type "Float (double-precision)"))
  (return (`self.DamageValue`)))

(fn `GetSectionIndex`
  (returns (SectionIndex :type Integer))
  (return (`self.CurrentSectionIndex`)))

(fn `LineTrace`
  (locals (Start :type "Vector Structure") (End :type "Vector Structure"))
  (bind _returnvalue (`self.K2_GetActorLocation`))
  (bind _followcamera (`self.FollowCamera`))
  (bind _returnvalue_2 (`SceneComponent.K2_GetComponentLocation` _followcamera))
  (switch `/Game/Blueprints/Characters/Sonny/Dream/E_GameplayType` (`self.GameplayType`)
    (:`NewEnumerator0`
      (set `local.Start` _returnvalue_2)
      (set `local.End` (+ _returnvalue_2 (* (`SceneComponent.GetForwardVector` _followcamera) 700.0))))
    (:`NewEnumerator2`
      (set `local.Start` _returnvalue)
      (set `local.End` (- (+ _returnvalue (* (`KismetMathLibrary.GetForwardVector` (`self.K2_GetActorRotation`)) 80.0)) (0.0 0.0 20.0)))))
  (bind _outhit (`KismetSystemLibrary.LineTraceSingle` :`Start` (`local.Start`) :`End` (`local.End`) :`TraceChannel` "TraceTypeQuery3" :`DrawDebugType` "ForOneFrame"))
  (bind (_bblockinghit _binitialoverlap _time _distance _location _impactpoint _normal _impactnormal _physmat _hitactor) (`GameplayStatics.BreakHitResult` _outhit))
  (if (`KismetSystemLibrary.DoesImplementInterface` _hitactor "/Game/Blueprints/Systems/Interaction/BPI_Interaction.BPI_Interaction_C")
    (if (not (== (`self.Hit Actor`) _hitactor))
      (bind _hit_actor (`self.Hit Actor`)
        (:`then`
          (message `/Game/Blueprints/Systems/Interaction/BPI_Interaction.HidePromt` _hit_actor))
        (:`else`
          _))
      (message `/Game/Blueprints/Systems/Interaction/BPI_Interaction.ShowPrompt` _hitactor)
      (set `self.Hit Actor` _hitactor)
      (return))
    (else
      (bind _hit_actor_2 (`self.Hit Actor`)
        (:`then`
          (message `/Game/Blueprints/Systems/Interaction/BPI_Interaction.HidePromt` _hit_actor_2))
        (:`else`
          _))
      (set `self.Hit Actor` null)
      (return))))

(fn `SetCameraPosition`
  (params (TargetArmLength :type "Float (double-precision)") (NewRotation :type "Rotator Structure"))
  (bind _cameraboom (`self.CameraBoom`))
  (`SceneComponent.K2_SetRelativeRotation` _cameraboom NewRotation false false)
  (set `SpringArmComponent.TargetArmLength` TargetArmLength _cameraboom))

(fn `SetControlls`
  (params (YawValue :type "Float (double-precision)"))
  (bind _cameraboom (`self.CameraBoom`))
  (bind _cameraboom_2 (`self.CameraBoom`))
  (switch `/Game/Blueprints/Characters/Sonny/Dream/E_GameplayType` (`self.GameplayType`)
    (:`NewEnumerator0`
      (set `self.bLineMode` false)
      (set `SpringArmComponent.bInheritYaw` true _cameraboom)
      (set `SpringArmComponent.bInheritPitch` true _cameraboom))
    (:`NewEnumerator1`
      (set `self.bLineMode` true :!label _label)
      (set `SpringArmComponent.bInheritYaw` false _cameraboom_2)
      (set `SpringArmComponent.bInheritPitch` false _cameraboom_2)
      (`Controller.SetControlRotation` (`GameplayStatics.GetPlayerController` 0) (`KismetMathLibrary.MakeRotator` 0.0 0.0 YawValue))
      (`self.K2_SetActorRotation` (`KismetMathLibrary.MakeRotator` 0.0 0.0 YawValue)))
    (:`NewEnumerator2`
      (goto _label))))

(fn `SpawnCombatBlock`
  (params (FloorActor :type "Actor Object Reference"))
  (bind (_returnvalue_x _returnvalue_y _returnvalue_z) (`KismetMathLibrary.BreakVector` (`self.K2_GetActorLocation` FloorActor)))
  (bind (_returnvalue_x_2 _returnvalue_y_2) (`KismetMathLibrary.BreakVector` (`KismetMathLibrary.Vector_SnappedToGrid` (`KismetMathLibrary.MakeVector` _returnvalue_x _returnvalue_y) 100.0)))
  (bind _canspawn (message `/Game/Blueprints/Systems/Combat/BPI_CombatFloor.CanSpawnBlock` FloorActor))
  (if _canspawn
    (message `/Game/Blueprints/Systems/Combat/BPI_CombatFloor.SetHasBlock` FloorActor true)
    (`|SpawnActorFromClass` "/Game/Blueprints/Systems/Combat/BP_CombatBlock.BP_CombatBlock_C" (`KismetMathLibrary.MakeTransform` (`KismetMathLibrary.MakeVector` _returnvalue_x_2 _returnvalue_y_2 (+ _returnvalue_z 70.0))) "AlwaysSpawn" "MultiplyWithRoot" null FloorActor null)))

(fn `UserConstructionScript`)