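; Sonny character for the intro reality sequence, who walks tagged spline paths and performs scripted turns.
; BeginPlay picks the first path and offsets the controller view; a Tick-fed Gate moves Sonny along the spline while open.
; Reaching the path end closes the gate and advances a StepIndex sequence of timeline turns and animation changes.
; Midway, StartMoving starts all intro NPCs and sends Sonny along the second path, ending in idle.
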(event `self.ReceiveBeginPlay`
  (bind _outactors (`GameplayStatics.GetAllActorsOfClassWithTag` "/Game/Blueprints/Characters/NPC/IntroReality/BP_IntroRealityPath.BP_IntroRealityPath_C" "sonny"))
  (set `self.Path` (`|GetArrayItem` _outactors))
  (`self.Path`
    (:`then`
      _)
    (:`else`
      _))
  (`self.AddControllerYawInput` 72.0)
  (`self.AddControllerPitchInput` 10.0))

(event `/Game/Blueprints/Characters/NPC/IntroReality/BPI_IntroRealityNPC.StartMoving`
  (bind _outactors (`GameplayStatics.GetAllActorsOfClass` "/Game/Blueprints/Characters/NPC/IntroReality/BP_IntroRealityNPC.BP_IntroRealityNPC_C"))
  (for _array_element _outactors
    (`/Game/Blueprints/Characters/NPC/IntroReality/BPI_IntroRealityNPC.StartMoving` _array_element))
  (bind _outactors_2 (`GameplayStatics.GetAllActorsOfClassWithTag` "/Game/Blueprints/Characters/NPC/IntroReality/BP_IntroRealityPath.BP_IntroRealityPath_C" "sonny2"))
  (set `self.Path` (`|GetArrayItem` _outactors_2))
  (`self.Path`
    (:`then`
      (`self.OpenGate`)
      (set `self.firstTime` false))
    (:`else`)))

(event `OpenGate`
  (bind _spline (`/Game/Blueprints/Characters/NPC/IntroReality/BP_IntroRealityPath.Spline` (`self.Path`)))
  (`SkeletalMeshComponent.PlayAnimation` (`self.Mesh`) "/Game/Characters/Mannequins/Animations/Manny/MM_Walk_Fwd.MM_Walk_Fwd" true)
  (goto _label :!via `Open`))

(event `CloseGate`
  (bind _spline (`/Game/Blueprints/Characters/NPC/IntroReality/BP_IntroRealityPath.Spline` (`self.Path`)))
  (goto _label :!via `Close`))

(event `self.ReceiveTick`
  (params (DeltaSeconds :type "Float (single-precision)"))
  (bind _spline (`/Game/Blueprints/Characters/NPC/IntroReality/BP_IntroRealityPath.Spline` (`self.Path`)))
  (`/Engine/EditorBlueprintResources/StandardMacros.Gate` true :!label _label
    (:`Exit`
      (bind _output_get (set `self.Distance` (+ (`self.Distance`) (* DeltaSeconds (`self.Speed`)))))
      (bind (_returnvalue_location _returnvalue_rotation) (`KismetMathLibrary.BreakTransform` (`SplineComponent.GetTransformAtDistanceAlongSpline` (`/Game/Blueprints/Characters/NPC/IntroReality/BP_IntroRealityPath.Spline` (`self.Path`)) _output_get "World" false)))
      (`self.K2_SetActorTransform` (`KismetMathLibrary.MakeTransform` _returnvalue_location _returnvalue_rotation))
      (if (`KismetMathLibrary.NearlyEqual_FloatFloat` (`self.Distance`) (`SplineComponent.GetDistanceAlongSplineAtSplinePoint` _spline (- (`SplineComponent.GetNumberOfSplinePoints` _spline) 1)) 10.0)
        (set `self.Distance` 0.0)
        (`self.CloseGate`)
        (`self.NextStep`)))))

(event `RotateNPC`
  (params (ZValue :type "Float (double-precision)"))
  (set `self.StartRotation` (`self.K2_GetActorRotation`))
  (bind (_direction _alpha) (`Timeline|Timeline` :!via `PlayFromStart`)
    (:`Update`
      (`self.K2_SetActorRelativeRotation` (`KismetMathLibrary.RLerp` (`self.StartRotation`) (`KismetMathLibrary.ComposeRotators` (`self.StartRotation`) (`KismetMathLibrary.MakeRotator` 0.0 0.0 ZValue)) _alpha)))
    (:`Finished`
      (`/Engine/EditorBlueprintResources/StandardMacros.IncrementInt` (`self.StepIndex`)
        (:`  `
          (`self.NextStep`))))))

(event `NextStep`
  (switch `int` (`self.StepIndex`)
    (:`0`
      (`SkeletalMeshComponent.PlayAnimation` (`self.Mesh`) "/Game/Characters/Mannequins/Animations/Manny/MM_Walk_InPlace.MM_Walk_InPlace" true)
      (`self.RotateNPC` -90.0))
    (:`1`
      (`KismetSystemLibrary.Delay` 1.0)
      (`/Game/Blueprints/Characters/NPC/IntroReality/BPI_IntroRealityNPC.StartMoving`)
      (`/Engine/EditorBlueprintResources/StandardMacros.IncrementInt` (`self.StepIndex`)))
    (:`2`
      (`self.RotateNPC` 90.0))
    (:`3`
      (`SkeletalMeshComponent.PlayAnimation` (`self.Mesh`) "/Game/Characters/Mannequins/Animations/Manny/MM_Idle.MM_Idle" true))))

(fn `UserConstructionScript`)