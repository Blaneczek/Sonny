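; BP_DataLayerSwitcherBox is a trigger volume that switches World Partition data layers when the player enters it.
; It caches the Data Layer Manager on BeginPlay, then reacts to box overlaps by the first player character only.
; On overlap it activates every layer in DataLayersToLoad and unloads every layer in DataLayersToUnload, non-recursively, with no reversal on exit.
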(event `self.ReceiveBeginPlay`
  (bind _returnvalue (`WorldPartitionBlueprintLibrary.GetDataLayerManager`)))

(event `self.Box.OnComponentBeginOverlap`
  (params (OverlappedComponent :type "PrimitiveComponent Object Reference") (OtherActor :type "Actor Object Reference") (OtherComp :type "PrimitiveComponent Object Reference") (OtherBodyIndex :type Integer) (bFromSweep :type Boolean) (SweepResult :type "HitResult Structure (by ref)"))
  (if (== OtherActor (`GameplayStatics.GetPlayerCharacter` 0))
    (for _array_element (`self.DataLayersToLoad`)
      (`DataLayerManager.SetDataLayerRuntimeState` (stale `self.ReceiveBeginPlay` _returnvalue) _array_element "Activated" false))
    (for _array_element_2 (`self.DataLayersToUnload`)
      (`DataLayerManager.SetDataLayerRuntimeState` (stale `self.ReceiveBeginPlay` _returnvalue) _array_element_2 "Unloaded" false))))

(fn `UserConstructionScript`)