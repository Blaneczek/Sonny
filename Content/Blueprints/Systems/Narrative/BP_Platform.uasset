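; BP_Platform is a moving platform that starts once when the player character steps into its Starter trigger.
; The overlap activates the InterpToMovement component and turns on collision for four blocker components.
; A fixed three-second delay, not a movement-finished event, then disables the blockers' collision again.
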(event `self.Starter.OnComponentBeginOverlap`
  (params (OverlappedComponent :type "PrimitiveComponent Object Reference") (OtherActor :type "Actor Object Reference") (OtherComp :type "PrimitiveComponent Object Reference") (OtherBodyIndex :type Integer) (bFromSweep :type Boolean) (SweepResult :type "HitResult Structure (by ref)"))
  (if (== OtherActor (`GameplayStatics.GetPlayerCharacter` 0))
    (`/Engine/EditorBlueprintResources/StandardMacros.DoOnce` false
      (:`Completed`
        (`self.SetBlockersCollisions` true)
        (`ActorComponent.Activate` (`self.InterpToMovement`) false)
        (`KismetSystemLibrary.Delay` 3.0)
        (`self.SetBlockersCollisions` false)))))

(fn `SetBlockersCollisions`
  (params (IsEnable :type Boolean))
  (if IsEnable
    (`PrimitiveComponent.SetCollisionEnabled` (`self.Blocker1`) "QueryAndPhysics")
    (`PrimitiveComponent.SetCollisionEnabled` (`self.Blocker2`) "QueryAndPhysics")
    (`PrimitiveComponent.SetCollisionEnabled` (`self.Blocker3`) "QueryAndPhysics")
    (`PrimitiveComponent.SetCollisionEnabled` (`self.Blocker4`) "QueryAndPhysics")
    (else
      (`PrimitiveComponent.SetCollisionEnabled` (`self.Blocker1`) "NoCollision")
      (`PrimitiveComponent.SetCollisionEnabled` (`self.Blocker2`) "NoCollision")
      (`PrimitiveComponent.SetCollisionEnabled` (`self.Blocker3`) "NoCollision")
      (`PrimitiveComponent.SetCollisionEnabled` (`self.Blocker4`) "NoCollision"))))

(fn `UserConstructionScript`)