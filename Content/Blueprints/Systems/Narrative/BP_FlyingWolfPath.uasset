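; Flying wolf path actor that sends a random BP_FlyingWolf from its side (left or right) flying along it.
; The Start event, or a delayed end overlap on its Box after a debug print, looks up wolves matching PlaceTag.
; It calls FlyYouFool on a random pick, passing itself as the path and the opposite side as the new tag.
; A delayed FindPath call is left unconnected.
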(event `Start`
  (bind _outactors (`GameplayStatics.GetAllActorsOfClassWithTag` "/Game/Blueprints/Characters/NPC/Dream/BP_FlyingWolf.BP_FlyingWolf_C" (`self.PlaceTag`) :!label _label))
  (bind _outitem (`KismetArrayLibrary.Array_Random` _outactors))
  (`/Engine/EditorBlueprintResources/StandardMacros.IsValid` _outitem
    (:`Is Valid`
      (switch `name` (`self.PlaceTag`)
        (:`right`
          (`/Game/Blueprints/Characters/NPC/Dream/BP_FlyingWolf.FlyYouFool` _outitem self "left"))
        (:`left`
          (`/Game/Blueprints/Characters/NPC/Dream/BP_FlyingWolf.FlyYouFool` _outitem self "right"))))))

(event `self.Box.OnComponentEndOverlap`
  (params (OverlappedComponent :type "PrimitiveComponent Object Reference") (OtherActor :type "Actor Object Reference") (OtherComp :type "PrimitiveComponent Object Reference") (OtherBodyIndex :type Integer))
  (`KismetSystemLibrary.Delay` 4.0)
  (`KismetSystemLibrary.PrintString` "Hello")
  (goto _label))

(fn `UserConstructionScript`)