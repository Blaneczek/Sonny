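; Interaction component that gives its owning actor a show/hide prompt and an interact event.
; On BeginPlay it caches the owner's WidgetComponent as the prompt.
; ShowPrompt reveals it and sets CanInteract while InteractionAvailable is true, also printing a debug string; HidePrompt reverses both.
; Interact stores its Multiple argument as future availability, fires OnInteract with CanInteract, then hides the prompt.
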(event `self.ReceiveBeginPlay`
  (`self.SetWidgetComponent`))

(fn `HidePrompt`
  (bind _widget (`self.Widget`))
  (`/Engine/EditorBlueprintResources/StandardMacros.IsValid` _widget
    (:`Is Valid`
      (`SceneComponent.SetVisibility` _widget false false)
      (set `self.CanInteract` false))))

(fn `Interact`
  (params (Multiple :type Boolean))
  (set `self.InteractionAvailable` Multiple)
  (`self.OnInteract` (`self.CanInteract`))
  (`self.HidePrompt`))

(fn `SetWidgetComponent`
  (set `self.Widget` (`Actor.GetComponentByClass` (`self.GetOwner`) "/Script/UMG.WidgetComponent")))

(fn `ShowPrompt`
  (bind _widget (`self.Widget`))
  (if (`self.InteractionAvailable`)
    (`/Engine/EditorBlueprintResources/StandardMacros.IsValid` _widget
      (:`Is Valid`
        (`SceneComponent.SetVisibility` _widget true false)
        (set `self.CanInteract` true)
        (`KismetSystemLibrary.PrintString` "dziala")))))