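; BP_SaveBox is a trigger volume that saves the game when the player walks into it.
; When the player character first overlaps its Box, a DoOnce sends save data to the GameInstance through a SaveGameDataMessage call and prints a confirmation.
; The save data holds the player's current transform, with the level reference fixed to Dream01Map and the NewGame flag set to true.
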(event `self.Box.OnComponentBeginOverlap`
  (params (OverlappedComponent :type "PrimitiveComponent Object Reference") (OtherActor :type "Actor Object Reference") (OtherComp :type "PrimitiveComponent Object Reference") (OtherBodyIndex :type Integer) (bFromSweep :type Boolean) (SweepResult :type "HitResult Structure (by ref)"))
  (if (== OtherActor (`GameplayStatics.GetPlayerCharacter` 0))
    (`/Engine/EditorBlueprintResources/StandardMacros.DoOnce` false
      (:`Completed`
        (message `/Game/Blueprints/Systems/Saves/BPI_SaveGame.SaveGameData` (`GameplayStatics.GetGameInstance`) (make `/Game/Blueprints/Systems/Saves/S_SaveData` true (make `SoftWorldReference` "/Game/Maps/Dreams/Dream01Map.Dream01Map") (`self.GetTransform` (`GameplayStatics.GetPlayerCharacter` 0))))
        (`KismetSystemLibrary.PrintString` "saved")))))

(fn `UserConstructionScript`)