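; BP_CombatStarter is a one-shot box trigger that starts combat gameplay for its assigned Level when the player overlaps it.
; BeginPlay tags the actor with its Level name.
; On overlap it enables the starting blocker's collision, sets the player's slowdown uses by level, and notifies the GameMode.
; It then broadcasts combat start to all BPI_Combat actors, passing its forward vector and location as reset point, and to every combat floor.
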(event `self.ReceiveBeginPlay`
  (`KismetArrayLibrary.Array_Add` (`self.Tags`) (`|GetEnumeratorName` (`self.Level`))))

(event `self.Box.OnComponentBeginOverlap`
  (params (OverlappedComponent :type "PrimitiveComponent Object Reference") (OtherActor :type "Actor Object Reference") (OtherComp :type "PrimitiveComponent Object Reference") (OtherBodyIndex :type Integer) (bFromSweep :type Boolean) (SweepResult :type "HitResult Structure (by ref)"))
  (bind _returnvalue (`GameplayStatics.GetPlayerCharacter` 0))
  (if (`self.bStarted`)
    _
    (elif (== OtherActor _returnvalue)
      (set `self.bStarted` true)
      (bind _returnvalue_2 (`GameplayStatics.GetActorOfClass` "/Game/Blueprints/Systems/Combat/BP_StartingBlocker.BP_StartingBlocker_C"))
      (`/Engine/EditorBlueprintResources/StandardMacros.IsValid` _returnvalue_2
        (:`Is Valid`
          (`/Game/Blueprints/Systems/Combat/BP_StartingBlocker.EnableCollision` _returnvalue_2))
        (:`Is Not Valid`
          _))
      (message `/Game/Blueprints/Systems/Combat/BPI_Combat.SetSlowdownUses` _returnvalue (select `/Game/Blueprints/Systems/E_GameplayLevel` (`self.Level`) :`NewEnumerator0` 1 :`NewEnumerator1` 2 :`NewEnumerator2` 3))
      (message `/Game/Blueprints/GameModes/Dreams/BPI_DreamGameMode.StartGameplayLevel` (`GameplayStatics.GetGameMode`) (`self.Level`) "NewEnumerator2")
      (bind _outactors (`GameplayStatics.GetAllActorsWithInterface` "/Game/Blueprints/Systems/Combat/BPI_Combat.BPI_Combat_C"))
      (for _array_element _outactors
        (message `/Game/Blueprints/Systems/Combat/BPI_Combat.StartCombat` _array_element (`self.GetActorForwardVector`) (`self.K2_GetActorLocation`) (`self.Level`)))
      (bind _outactors_2 (`GameplayStatics.GetAllActorsOfClass` "/Game/Blueprints/Systems/Combat/BP_CombatFloor.BP_CombatFloor_C"))
      (for _array_element_2 _outactors_2
        (message `/Game/Blueprints/Systems/Combat/BPI_CombatFloor.StartCombat` _array_element_2)))))

(fn `UserConstructionScript`)