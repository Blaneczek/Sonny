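; Combat floor tile that shows whether a block can be spawned on it and can randomly turn into a slowing tile.
; Cursor hover during combat, combatant overlap, Sonny's range, block occupancy and block supply set flags.
; ChangeFloorColor turns those flags into overlay materials and updates CanSpawn, which CanSpawnBlock exposes.
; DrawSlowFloor rolls a timed slow state, and SlowedBox overlaps notify the player character when slowing starts or ends.
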(event `/Game/Blueprints/Systems/Combat/BPI_CombatFloor.FinishCombat`
  (set `self.bCombat` false))

(event `/Game/Blueprints/Systems/Combat/BPI_CombatFloor.StartCombat`
  (set `self.bCombat` true))

(event `self.StaticMeshComponent.OnBeginCursorOver`
  (params (TouchedComponent :type "PrimitiveComponent Object Reference"))
  (if (`self.bCombat`)
    (set `self.bHovered` true)
    (`self.ChangeFloorColor`)))

(event `self.StaticMeshComponent.OnEndCursorOver`
  (params (TouchedComponent :type "PrimitiveComponent Object Reference"))
  (if (`self.bCombat`)
    (set `self.bHovered` false)
    (`self.ChangeFloorColor`)))

(event `self.Box.OnComponentBeginOverlap`
  (params (OverlappedComponent :type "PrimitiveComponent Object Reference") (OtherActor :type "Actor Object Reference") (OtherComp :type "PrimitiveComponent Object Reference") (OtherBodyIndex :type Integer) (bFromSweep :type Boolean) (SweepResult :type "HitResult Structure (by ref)"))
  (if (`KismetSystemLibrary.DoesImplementInterface` OtherActor "/Game/Blueprints/Systems/Combat/BPI_Combat.BPI_Combat_C")
    (set `self.bStepOn` true)
    (`self.ChangeFloorColor`)))

(event `self.Box.OnComponentEndOverlap`
  (params (OverlappedComponent :type "PrimitiveComponent Object Reference") (OtherActor :type "Actor Object Reference") (OtherComp :type "PrimitiveComponent Object Reference") (OtherBodyIndex :type Integer))
  (if (`KismetSystemLibrary.DoesImplementInterface` OtherActor "/Game/Blueprints/Systems/Combat/BPI_Combat.BPI_Combat_C")
    (set `self.bStepOn` false)
    (`self.ChangeFloorColor`)))

(event `/Game/Blueprints/Systems/Combat/BPI_CombatFloor.SonnyInRange`
  (set `self.bInRange` true)
  (`self.ChangeFloorColor`))

(event `/Game/Blueprints/Systems/Combat/BPI_CombatFloor.SonnyOutRange`
  (set `self.bInRange` false)
  (`self.ChangeFloorColor`))

(event `/Game/Blueprints/Systems/Combat/BPI_CombatFloor.SetHasBlock`
  (params (HasBlock :type Boolean))
  (set `self.bHasBlock` HasBlock)
  (`self.ChangeFloorColor`))

(event `/Game/Blueprints/Systems/Combat/BPI_CombatFloor.Reset`
  (set `self.bHasBlock` false)
  (set `self.bHovered` false)
  (set `self.bStepOn` false)
  (set `self.bCanSpawn` false)
  (`self.ChangeFloorColor`))

(event `/Game/Blueprints/Systems/Combat/BPI_CombatFloor.DrawSlowFloor`
  (if (<= (`KismetMathLibrary.RandomIntegerInRange` 0 100) 15)
    (set `self.bSlowFloor` true)
    (`self.ChangeFloorColor`)
    (`KismetSystemLibrary.K2_SetTimerDelegate` (delegate `CancelSlowFloor`) (`self.SlowFlowDuration`))))

(event `CancelSlowFloor`
  (set `self.bSlowFloor` false)
  (`self.ChangeFloorColor`)
  (if (`self.bPlayerSlowed`)
    (set `self.bPlayerSlowed` false)
    (message `/Game/Blueprints/Systems/Combat/BPI_Combat.SlowDown` (`GameplayStatics.GetPlayerCharacter` 0) false)))

(event `/Game/Blueprints/Systems/Combat/BPI_CombatFloor.IsNoMoreBlocks`
  (params (NoMore :type Boolean))
  (set `self.bNoMoreBlocks` NoMore))

(event `self.SlowedBox.OnComponentBeginOverlap`
  (params (OverlappedComponent :type "PrimitiveComponent Object Reference") (OtherActor :type "Actor Object Reference") (OtherComp :type "PrimitiveComponent Object Reference") (OtherBodyIndex :type Integer) (bFromSweep :type Boolean) (SweepResult :type "HitResult Structure (by ref)"))
  (if (and (== OtherActor (`GameplayStatics.GetPlayerCharacter` 0)) (`self.bSlowFloor`))
    (set `self.bPlayerSlowed` true)
    (message `/Game/Blueprints/Systems/Combat/BPI_Combat.SlowDown` (`GameplayStatics.GetPlayerCharacter` 0) true)))

(event `self.SlowedBox.OnComponentEndOverlap`
  (params (OverlappedComponent :type "PrimitiveComponent Object Reference") (OtherActor :type "Actor Object Reference") (OtherComp :type "PrimitiveComponent Object Reference") (OtherBodyIndex :type Integer))
  (if (and (== OtherActor (`GameplayStatics.GetPlayerCharacter` 0)) (`self.bSlowFloor`))
    (set `self.bPlayerSlowed` false)
    (message `/Game/Blueprints/Systems/Combat/BPI_Combat.SlowDown` (`GameplayStatics.GetPlayerCharacter` 0) false)))

(fn `CanSpawnBlock`
  (returns (CanSpawn :type Boolean))
  (return (and (`self.bCanSpawn`) (not (`self.bHasBlock`)))))

(fn `ChangeFloorColor`
  (bind _staticmeshcomponent (`self.StaticMeshComponent`))
  (bind _staticmeshcomponent_2 (`self.StaticMeshComponent`))
  (if (`self.bHasBlock`)
    (`MeshComponent.SetOverlayMaterial` (`self.StaticMeshComponent`) (`self.HoveredOverlayRed`))
    (return)
    (elif (`self.bInRange`)
      (if (`self.bHovered`)
        (if (`self.bStepOn`)
          _
          (elif (`self.bNoMoreBlocks`)
            _
            (else
              (`MeshComponent.SetOverlayMaterial` _staticmeshcomponent_2 (`self.HoveredOverlayGreen`))
              (set `self.bCanSpawn` true)
              (return))))
        (`MeshComponent.SetOverlayMaterial` _staticmeshcomponent_2 (`self.HoveredOverlayRed`))
        (set `self.bCanSpawn` false)
        (return)
        (else
          (`MeshComponent.SetOverlayMaterial` (`self.StaticMeshComponent`) (`self.DefaultOverlay`))
          (if (`self.bSlowFloor`)
            (`MeshComponent.SetOverlayMaterial` (`self.StaticMeshComponent`) (`self.HoveredOverlaySlow`))
            (return)
            (else
              (return)))))
      (elif (`self.bHovered`)
        (`MeshComponent.SetOverlayMaterial` _staticmeshcomponent (`self.HoveredOverlayRed`))
        (set `self.bCanSpawn` false)
        (return)
        (else
          (`MeshComponent.SetOverlayMaterial` _staticmeshcomponent null)
          (if (`self.bSlowFloor`)
            (`MeshComponent.SetOverlayMaterial` (`self.StaticMeshComponent`) (`self.HoveredOverlaySlow`))
            (return)
            (else
              (return))))))))

(fn `UserConstructionScript`)