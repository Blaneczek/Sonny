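; Interactable block that gates combat sections, showing its remaining HP as text and losing one point per interaction through the interaction component.
; Each hit briefly swaps the cube material and restarts a looping one-second timer, which restores full HP after about three seconds without another hit.
; At zero HP it sends SectionChangeMessage with the next section index to every BPI_Combat actor, then destroys itself.
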(event `self.ShowPrompt`
  (`/Game/Blueprints/Systems/Interaction/BPC_Interaction.ShowPrompt` (`self.BPC_Interaction`)))

(event `self.HidePromt`
  (`/Game/Blueprints/Systems/Interaction/BPC_Interaction.HidePrompt` (`self.BPC_Interaction`)))

(event `self.OnInteract`
  (params (Actor :type "Actor Object Reference"))
  (`/Game/Blueprints/Systems/Interaction/BPC_Interaction.Interact` (`self.BPC_Interaction`) true)
  (`/Engine/EditorBlueprintResources/StandardMacros.IsValid` self
    (:`Is Valid`
      (`self.ShowPrompt`))))

(event `self.BPC_Interaction.OnInteract`
  (params (CanInteract :type Boolean))
  (if CanInteract
    (`self.StartTimer`)
    (bind _result (`/Engine/EditorBlueprintResources/StandardMacros.DecrementInt` (`self.CurrentHP`))
      (:`  `
        (if (== _result 0)
          (bind _outactors (`GameplayStatics.GetAllActorsWithInterface` "/Game/Blueprints/Systems/Combat/BPI_Combat.BPI_Combat_C"))
          (for _array_element _outactors
            (message `/Game/Blueprints/Systems/Combat/BPI_Combat.SectionChange` _array_element (+ (`self.SectionIndex`) 1)))
          (`self.K2_DestroyActor`)
          (else
            (`TextRenderComponent.K2_SetText` (`self.TextRender`) (`KismetTextLibrary.Conv_IntToText` (`self.CurrentHP`)))
            (`PrimitiveComponent.SetMaterial` (`self.Cube`) 0 "/Engine/BasicShapes/BasicShapeMaterial_Inst.BasicShapeMaterial_Inst")
            (`KismetSystemLibrary.Delay` 0.1)
            (`PrimitiveComponent.SetMaterial` (`self.Cube`) 0 "/Engine/EngineMaterials/NaniteHiddenSectionMaterial.NaniteHiddenSectionMaterial")))))))

(event `/Game/Blueprints/Systems/Combat/BPI_Combat.StartCombat`
  (params (ForwardVector :type "Vector Structure"))
  (`self.StartTimer`))

(event `StartTimer`
  (set `self.Time` 0.0)
  (bind _returnvalue (`KismetSystemLibrary.K2_SetTimerDelegate` (delegate `Clock`) 1.0 true))
  (set `self.Timer` _returnvalue))

(event `Clock`
  (bind _result (`/Engine/EditorBlueprintResources/StandardMacros.IncrementFloat` (`self.Time`))
    (:`  `
      (if (>= _result 3.0)
        (set `self.CurrentHP` (`self.HP`))
        (`TextRenderComponent.K2_SetText` (`self.TextRender`) (`KismetTextLibrary.Conv_IntToText` (`self.HP`)))
        (`KismetSystemLibrary.K2_ClearAndInvalidateTimerHandle` (`self.Timer`))))))

(fn `GetAttackDamageValue`
  (returns (Value :type "Float (double-precision)"))
  (return 0.0))

(fn `GetSectionIndex`
  (returns (SectionIndex :type Integer))
  (return 0))

(fn `UserConstructionScript`)