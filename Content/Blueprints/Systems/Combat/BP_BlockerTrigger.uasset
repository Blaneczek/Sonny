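; BP_BlockerTrigger is a box trigger that activates a tagged blocker when the player enters it.
; When the player character overlaps the box, it finds BP_Blocker actors matching its Tag and calls EnableCollision on the first valid one.
; A separate ResetCollision function sets the box's Pawn channel response back to Overlap.
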(event `self.Box.OnComponentBeginOverlap`
  (params (OverlappedComponent :type "PrimitiveComponent Object Reference") (OtherActor :type "Actor Object Reference") (OtherComp :type "PrimitiveComponent Object Reference") (OtherBodyIndex :type Integer) (bFromSweep :type Boolean) (SweepResult :type "HitResult Structure (by ref)"))
  (if (== OtherActor (`GameplayStatics.GetPlayerCharacter` 0))
    (bind _outactors (`GameplayStatics.GetAllActorsOfClassWithTag` "/Game/Blueprints/Systems/Combat/BP_Blocker.BP_Blocker_C" (`self.Tag`)))
    (bind _output (`|GetArrayItem` _outactors))
    (`/Engine/EditorBlueprintResources/StandardMacros.IsValid` _output
      (:`Is Valid`
        (`/Game/Blueprints/Systems/Combat/BP_Blocker.EnableCollision` _output)))))

(fn `ResetCollision`
  (`PrimitiveComponent.SetCollisionResponseToChannel` (`self.Box`) "ECC_Pawn" "ECR_Overlap"))

(fn `UserConstructionScript`)