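; BP_CombatEnd is a trigger volume that ends combat when the player overlaps its box.
; On first overlap it sends finish-combat messages to all BP_CombatFloor actors and BPI_Combat implementers, notifies the game mode that the gameplay level ended, and disables its own collision.
; It then enables collision on the first BP_Blocker found with the matching Tag.
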(event `self.Box.OnComponentBeginOverlap`
  (params (OverlappedComponent :type "PrimitiveComponent Object Reference") (OtherActor :type "Actor Object Reference") (OtherComp :type "PrimitiveComponent Object Reference") (OtherBodyIndex :type Integer) (bFromSweep :type Boolean) (SweepResult :type "HitResult Structure (by ref)"))
  (if (== OtherActor (`GameplayStatics.GetPlayerCharacter` 0))
    (`/Engine/EditorBlueprintResources/StandardMacros.DoOnce` false
      (:`Completed`
        (`self.UnblockEnd`)
        (bind _outactors (`GameplayStatics.GetAllActorsOfClassWithTag` "/Game/Blueprints/Systems/BP_Blocker.BP_Blocker_C" (`self.Tag`)))
        (bind _output (`|GetArrayItem` _outactors))
        (`/Engine/EditorBlueprintResources/StandardMacros.IsValid` _output
          (:`Is Valid`
            (`/Game/Blueprints/Systems/BP_Blocker.EnableCollision` _output)))))))

(fn `UnblockEnd`
  (bind _outactors (`GameplayStatics.GetAllActorsOfClass` "/Game/Blueprints/Systems/Combat/BP_CombatFloor.BP_CombatFloor_C"))
  (for _array_element _outactors
    (message `/Game/Blueprints/Systems/Combat/BPI_CombatFloor.FinishCombat` _array_element))
  (bind _outactors_2 (`GameplayStatics.GetAllActorsWithInterface` "/Game/Blueprints/Systems/Combat/BPI_Combat.BPI_Combat_C"))
  (for _array_element_2 _outactors_2
    (`/Engine/EditorBlueprintResources/StandardMacros.IsValid` _array_element_2
      (:`Is Valid`
        (message `/Game/Blueprints/Systems/Combat/BPI_Combat.FinishCombat` _array_element_2))))
  (message `/Game/Blueprints/GameModes/Dreams/BPI_DreamGameMode.EndGameplayLevel` (`GameplayStatics.GetGameMode`))
  (`PrimitiveComponent.SetCollisionEnabled` (`self.Box`) "NoCollision"))

(fn `UserConstructionScript`)