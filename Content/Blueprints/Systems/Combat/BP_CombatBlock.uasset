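; BP_CombatBlock is a destructible block for the combat mode, with mesh, material and transform chosen per level at BeginPlay.
; Interactions take the attacker's damage value and route through BPCInteraction to reduce HP; non-player attackers force CanInteract and start a timer restoring starting HP.
; At zero HP it notifies the attacker, hides, then clears the floor's block flag and destroys itself after a delay.
; ResetCombat resets the floor and destroys the block.
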(event `self.ReceiveBeginPlay`
  (bind _cube (`self.Cube`))
  (bind _cube_2 (`self.Cube`))
  (bind _cube_3 (`self.Cube`))
  (switch `/Game/Blueprints/Systems/E_GameplayLevel` (`self.Level`)
    (:`NewEnumerator0`
      (`SceneComponent.K2_SetRelativeLocation` _cube_2 (0.0 0.0 -50.0) false false)
      (`SceneComponent.SetRelativeScale3D` _cube_2 (0.55 0.53 1.05))
      (`StaticMeshComponent.SetStaticMesh` _cube_2 "/Game/Assets/FantasyBundle/Meshes/SM_WoodStairs02.SM_WoodStairs02")
      (`PrimitiveComponent.SetMaterial` (`self.Cube`) 0 "/Game/Assets/FantasyBundle/Materials/MI_WoodDetails1.MI_WoodDetails1"))
    (:`NewEnumerator1`
      (`SceneComponent.K2_SetRelativeLocation` _cube_3 (0.0 0.0 0.0) false false)
      (`SceneComponent.SetRelativeScale3D` _cube_3 (1.5 2.05 3.0775))
      (`StaticMeshComponent.SetStaticMesh` _cube_3 "/Game/Assets/GothicTemple/Environment/Props/GothicBlocks/SM_GothicBlock_05.SM_GothicBlock_05")
      (`PrimitiveComponent.SetMaterial` (`self.Cube`) 0 "/Game/Assets/GothicTemple/Environment/Props/GothicBlocks/MI_TempleAssetsBlocks3.MI_TempleAssetsBlocks3"))
    (:`NewEnumerator2`
      (`SceneComponent.K2_SetRelativeLocation` _cube (0.0 0.0 -58.0) false false)
      (`SceneComponent.SetRelativeScale3D` _cube (11.0 11.0 11.95))
      (`StaticMeshComponent.SetStaticMesh` _cube "/Game/Megascans/3D_Assets/Urban_Street_Cobblestone_Lava_Single_xb0eddt/S_Urban_Street_Cobblestone_Lava_Single_xb0eddt_lod5_Var1.S_Urban_Street_Cobblestone_Lava_Single_xb0eddt_lod5_Var1")
      (`PrimitiveComponent.SetMaterial` (`self.Cube`) 0 "/Game/Assets/Level03/MS/3D/Massive_Nordic_Coastal_Cliff_veqnci0db/Smart/MI_veqnci0db_Smart3.MI_veqnci0db_Smart3")))
  (message `/Game/Blueprints/GameModes/Dreams/BPI_DreamGameMode.UpdateCombatModeScore` (`GameplayStatics.GetGameMode`) "NewEnumerator7")
  (set `self.StarterHP` (`self.HP`)))

(event `/Game/Blueprints/Systems/Interaction/BPI_Interaction.ShowPrompt`
  (`/Game/Blueprints/Systems/Interaction/BPC_Interaction.ShowPrompt` (`self.BPC_Interaction`)))

(event `/Game/Blueprints/Systems/Interaction/BPI_Interaction.HidePromt`
  (`/Game/Blueprints/Systems/Interaction/BPC_Interaction.HidePrompt` (`self.BPC_Interaction`)))

(event `/Game/Blueprints/Systems/Interaction/BPI_Interaction.OnInteract`
  (params (Actor :type "Actor Object Reference"))
  (bind _output_get (set `self.AttackerActor` Actor))
  (bind _value (message `/Game/Blueprints/Systems/Combat/BPI_Combat.GetAttackDamageValue` _output_get))
  (set `self.DamageValue` _value)
  (if (== Actor (`GameplayStatics.GetPlayerCharacter` 0))
    (`/Game/Blueprints/Systems/Interaction/BPC_Interaction.Interact` (`self.BPC_Interaction`) true)
    (`/Engine/EditorBlueprintResources/StandardMacros.IsValid` self
      (:`Is Valid`
        (`self.ShowPrompt`)))
    (else
      (set `/Game/Blueprints/Systems/Interaction/BPC_Interaction.CanInteract` true (`self.BPC_Interaction`))
      (`/Game/Blueprints/Systems/Interaction/BPC_Interaction.Interact` (`self.BPC_Interaction`) true)
      (`KismetSystemLibrary.K2_SetTimerDelegate` (delegate `RestoreHealth`) 4.0))))

(event `RestoreHealth`
  (set `self.HP` (`self.StarterHP`)))

(event `self.BPC_Interaction.OnInteract`
  (params (CanInteract :type Boolean))
  (if CanInteract
    (bind _output_get (set `self.HP` (- (`self.HP`) (`self.DamageValue`))))
    (if (<= _output_get 0.0)
      (message `/Game/Blueprints/Systems/Combat/BPI_Combat.BlockDestroyed` (`self.AttackerActor`))
      (`self.SetActorHiddenInGame` true)
      (`self.SetActorEnableCollision` false)
      (`KismetSystemLibrary.Delay` 2.0)
      (message `/Game/Blueprints/Systems/Combat/BPI_CombatFloor.SetHasBlock` (`self.FloorActor`) false)
      (`self.K2_DestroyActor`))))

(event `/Game/Blueprints/Systems/Combat/BPI_Combat.ResetCombat`
  (bind _flooractor (`self.FloorActor`))
  (`/Engine/EditorBlueprintResources/StandardMacros.IsValid` _flooractor
    (:`Is Valid`
      (message `/Game/Blueprints/Systems/Combat/BPI_CombatFloor.Reset` _flooractor))
    (:`Is Not Valid`
      _))
  (`self.K2_DestroyActor`))

(fn `GetAttackDamageValue`
  (returns (Value :type "Float (double-precision)"))
  (return 0.0))

(fn `GetNumberOfSlowdownUses`
  (returns (Uses :type Integer))
  (return 0))

(fn `GetSectionIndex`
  (returns (SectionIndex :type Integer))
  (return 0))

(fn `UserConstructionScript`)