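; BP_LineBlock is one block in the IntroLines line-path system, where a path advances block by block through available neighbors.
; HighlightBlock fires once on an available block, changing its material, marking the previous block, closing that block's paths and opening its own unmarked neighbors.
; GetNeighborBlocks finds adjacent blocks with box overlaps along the forward and up axes, deduplicated through a set.
; A dead-end debug print is left unconnected.
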(event `/Game/Blueprints/Systems/IntroLines/BPI_Lines.HighlightBlock`
  (params (PreviousBlock :type "Actor Object Reference"))
  (if (`self.bAvailable`)
    (`/Engine/EditorBlueprintResources/StandardMacros.DoOnce` false
      (:`Completed`
        (message `/Game/Blueprints/Systems/IntroLines/BPI_Lines.MarkBlock` PreviousBlock)
        (`PrimitiveComponent.SetMaterial` (`self.Cube`) 0 "/Engine/MapTemplates/Materials/BasicAsset03.BasicAsset03")
        (message `/Game/Blueprints/Systems/IntroLines/BPI_Lines.BlockPreviousPaths` PreviousBlock)
        (for _array_element (`self.NeighborBlocks`)
          (`/Engine/EditorBlueprintResources/StandardMacros.IsValid` _array_element
            (:`Is Valid`
              (bind _asbp_line_block (cast `/Game/Blueprints/Systems/IntroLines/BP_LineBlock` _array_element))
              (if (not (`/Game/Blueprints/Systems/IntroLines/BP_LineBlock.bMarked` _asbp_line_block))
                (set `/Game/Blueprints/Systems/IntroLines/BP_LineBlock.bAvailable` true _asbp_line_block)))))))))

(event `/Game/Blueprints/Systems/IntroLines/BPI_Lines.BlockPreviousPaths`
  (for _array_element (`self.NeighborBlocks`)
    (`/Engine/EditorBlueprintResources/StandardMacros.IsValid` _array_element
      (:`Is Valid`
        (bind _asbp_line_block (cast `/Game/Blueprints/Systems/IntroLines/BP_LineBlock` _array_element))
        (set `/Game/Blueprints/Systems/IntroLines/BP_LineBlock.bAvailable` false _asbp_line_block)))))

(event `GetNeighborBlocks`
  (`KismetArrayLibrary.Array_Clear` (`self.NeighborBlocks`))
  (`BlueprintSetLibrary.Set_Clear` (`self.tempSet`))
  (bind _outactors (`KismetSystemLibrary.BoxOverlapActors` (`self.K2_GetActorLocation`) (`KismetMathLibrary.Vector_GetAbs` (* 25.0 (`self.GetActorForwardVector`))) (`|MakeArray` "ObjectTypeQuery5" :!type "EObjectTypeQuery Enum") "BP_LineBlock_C" (`|MakeArray` self :!type "Actor Object Reference")))
  (`BlueprintSetLibrary.Set_AddItems` (`self.tempSet`) _outactors)
  (bind _outactors_2 (`KismetSystemLibrary.BoxOverlapActors` (`self.K2_GetActorLocation`) (`KismetMathLibrary.Vector_GetAbs` (* 25.0 (`self.GetActorUpVector`))) (`|MakeArray` "ObjectTypeQuery5" :!type "EObjectTypeQuery Enum") "BP_LineBlock_C" (`|MakeArray` self :!type "Actor Object Reference")))
  (`BlueprintSetLibrary.Set_AddItems` (`self.tempSet`) _outactors_2)
  (bind _result (`BlueprintSetLibrary.Set_ToArray` (`self.tempSet`)))
  (set `self.NeighborBlocks` _result))

(fn `IsAvailable`
  (returns (Available :type Boolean))
  (return (`self.bAvailable`)))

(fn `MarkBlock`
  (`/Engine/EditorBlueprintResources/StandardMacros.DoOnce` false
    (:`Completed`
      (`PrimitiveComponent.SetMaterial` (`self.Cube`) 0 "/Engine/MapTemplates/Materials/BasicAsset01.BasicAsset01")
      (set `self.bAvailable` false)
      (set `self.bMarked` true))))

(fn `UserConstructionScript`)