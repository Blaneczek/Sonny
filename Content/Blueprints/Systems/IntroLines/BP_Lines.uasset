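; BP_Lines is a spline actor that builds a line of deformed spline meshes along its path, apparently for the intro lines system.
; The construction script calls GenerateMesh, which clears the array and adds X-forward spline mesh components attached to the spline, fitting each to local positions and tangents by distance.
; Section length scales with MeshLength and actor X scale, and only whole sections are built, leaving any remainder uncovered.
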(event `GenerateMesh`
  (bind _returnvalue_x (`KismetMathLibrary.BreakVector` (`self.GetActorScale3D`)))
  (bind _spline (`self.Spline`))
  (`KismetArrayLibrary.Array_Clear` (`self.SplineMeshes`))
  (set `self.SectionLength` (* _returnvalue_x (* (`self.MeshLength`) 10.0)))
  (for _index (range (`KismetMathLibrary.FTrunc` (/ (`SplineComponent.GetSplineLength` (`self.Spline`)) (`self.SectionLength`))))
    (bind _returnvalue (`AddComponent|NODE_AddSplineMeshComponent-0`))
    (`KismetArrayLibrary.Array_Set` (`self.SplineMeshes`) _index _returnvalue true)
    (`SplineMeshComponent.SetForwardAxis` _returnvalue "X" true)
    (`SceneComponent.K2_AttachToComponent` _returnvalue (`self.Spline`) "None" "KeepRelative" "KeepRelative" "KeepRelative" true)
    (bind _returnvalue_2 (* _index (`self.SectionLength`)))
    (bind _returnvalue_3 (* (+ _index 1) (`self.SectionLength`)))
    (`SplineMeshComponent.SetStartAndEnd` _returnvalue (`SplineComponent.GetLocationAtDistanceAlongSpline` _spline _returnvalue_2 "Local") (`SplineComponent.GetTangentAtDistanceAlongSpline` _spline _returnvalue_2 "Local") (`SplineComponent.GetLocationAtDistanceAlongSpline` _spline _returnvalue_3 "Local") (`SplineComponent.GetTangentAtDistanceAlongSpline` _spline _returnvalue_3 "Local") true)))

(fn `UserConstructionScript`
  (`self.GenerateMesh`))