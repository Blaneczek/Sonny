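; BP_LinesCreatorDream is a spline-based placer that builds rows of BP_LineBlockDream actors for the Dream variant of Line Mode.
; SpawnAllCreators clears every existing block, then has each creator in the level spawn blocks at even intervals along its spline.
; Spacing comes from mesh length and actor X scale, and blocks take the creator's rotation rather than following the spline's.
; A separate ConnectBlocks function has every block find its neighbours.
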(event `SpawnAllCreators`
  (`self.DestroyAllBlocks`)
  (bind _outactors (`GameplayStatics.GetAllActorsOfClass` "BP_LinesCreatorDream_C"))
  (for _array_element _outactors
    (`self.SpawnBlocks` _array_element)))

(event `SpawnBlocks`
  (bind _returnvalue_x (`KismetMathLibrary.BreakVector` (`self.GetActorScale3D`)))
  (set `self.SectionLength` (* _returnvalue_x (`self.MeshLength`)))
  (for _index (range (`KismetMathLibrary.FFloor` (/ (`SplineComponent.GetSplineLength` (`self.Spline`)) (`self.SectionLength`))))
    (`|SpawnActorFromClass` "/Game/Blueprints/Systems/LineMode/Dream/BP_LineBlockDream.BP_LineBlockDream_C" (`KismetMathLibrary.MakeTransform` (`SplineComponent.GetLocationAtDistanceAlongSpline` (`self.Spline`) (+ (* _index (`self.SectionLength`)) (* (`self.MeshLength`) 0.5)) "World") (`self.K2_GetActorRotation`) (`KismetMathLibrary.MakeVector` (* (`self.MeshLength`) 0.01) 1.0 1.0)) "AlwaysSpawn" "MultiplyWithRoot" null null)))

(fn `ConnectBlocks`
  (bind _outactors (`GameplayStatics.GetAllActorsOfClass` "/Game/Blueprints/Systems/LineMode/Dream/BP_LineBlockDream.BP_LineBlockDream_C"))
  (for _array_element _outactors
    (`/Game/Blueprints/Systems/LineMode/Dream/BP_LineBlockDream.GetNeighborBlocks` _array_element)))

(fn `DestroyAllBlocks`
  (bind _outactors (`GameplayStatics.GetAllActorsOfClass` "/Game/Blueprints/Systems/LineMode/Dream/BP_LineBlockDream.BP_LineBlockDream_C"))
  (for _array_element _outactors
    (`self.K2_DestroyActor` _array_element)))

(fn `UserConstructionScript`)