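; BP_LineModeStarter is a one-shot trigger that starts Dream line-mode gameplay when the player character overlaps its box.
; On overlap it notifies the game mode, then has every BP_LineBlockDream remove overlapping boxes and find its neighbors.
; It then sends all BPI_LineModeDream actors the level, using its own location and forward vector as reset point and direction.
; Shortly after BeginPlay, it also resets all block colors.
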(event `self.ReceiveBeginPlay`
  (`KismetSystemLibrary.Delay` 0.2)
  (bind _outactors (`GameplayStatics.GetAllActorsOfClass` "/Game/Blueprints/Systems/LineMode/Dream/BP_LineBlockDream.BP_LineBlockDream_C"))
  (for _array_element _outactors
    (message `/Game/Blueprints/Systems/LineMode/BPI_Lines.ResetColors` _array_element)))

(event `self.Box.OnComponentBeginOverlap`
  (params (OverlappedComponent :type "PrimitiveComponent Object Reference") (OtherActor :type "Actor Object Reference") (OtherComp :type "PrimitiveComponent Object Reference") (OtherBodyIndex :type Integer) (bFromSweep :type Boolean) (SweepResult :type "HitResult Structure (by ref)"))
  (if (`self.bStarted`)
    _
    (elif (== OtherActor (`GameplayStatics.GetPlayerCharacter` 0))
      (set `self.bStarted` true)
      (message `/Game/Blueprints/GameModes/Dreams/BPI_DreamGameMode.StartGameplayLevel` (`GameplayStatics.GetGameMode`) (`self.Level`) "NewEnumerator1")
      (bind _outactors (`GameplayStatics.GetAllActorsOfClass` "/Game/Blueprints/Systems/LineMode/Dream/BP_LineBlockDream.BP_LineBlockDream_C"))
      (for _array_element _outactors
        (`/Engine/EditorBlueprintResources/StandardMacros.IsValid` _array_element
          (:`Is Valid`
            (message `/Game/Blueprints/Systems/LineMode/BPI_Lines.RemoveOverlappingBoxes ` _array_element)
            (`/Game/Blueprints/Systems/LineMode/Dream/BP_LineBlockDream.GetNeighborBlocks` _array_element))))
      (bind _outactors_2 (`GameplayStatics.GetAllActorsWithInterface` "/Game/Blueprints/Systems/LineMode/Dream/BPI_LineModeDream.BPI_LineModeDream_C"))
      (for _array_element_2 _outactors_2
        (`/Engine/EditorBlueprintResources/StandardMacros.IsValid` _array_element_2
          (:`Is Valid`
            (message `/Game/Blueprints/Systems/LineMode/Dream/BPI_LineModeDream.LineModeSetup` _array_element_2 (`self.GetActorForwardVector`) (`self.Level`) (`self.K2_GetActorLocation`))))))))

(fn `UserConstructionScript`)