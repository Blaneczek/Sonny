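; Interactable level selector for Line Mode that labels itself with its target level and moves the player there.
; Its prompt fills a world widget with that level's best score and score thresholds from the GameMode.
; Interacting shows the line death screen, unloads the current level's Data Layer and activates the target's (only Level01 and Level02 are mapped).
; After a short delay it resets BP_LineModeStarter and relocates the player onto it.
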(event `self.ReceiveBeginPlay`
  (`TextRenderComponent.K2_SetText` (`self.TextRender`) (`KismetTextLibrary.Conv_StringToText` (`|GetEnumeratorNameAsString` (`self.DesiredLevel`)))))

(event `/Game/Blueprints/Systems/Interaction/BPI_Interaction.HidePromt`
  (`/Game/Blueprints/Systems/Interaction/BPC_Interaction.HidePrompt` (`self.BPC_Interaction`)))

(event `/Game/Blueprints/Systems/Interaction/BPI_Interaction.ShowPrompt`
  (bind _aswbp_score_levels_on_map (cast `/Game/Blueprints/UI/Gameplay/WBP_ScoreLevelsOnMap` (`WidgetComponent.GetUserWidgetObject` (`self.Widget`))))
  (`/Engine/EditorBlueprintResources/StandardMacros.IsValid` _aswbp_score_levels_on_map
    (:`Is Valid`
      (bind (_bestscore _scorelevels) (message `/Game/Blueprints/GameModes/Dreams/BPI_DreamGameMode.GetScores` (`GameplayStatics.GetGameMode`) "NewEnumerator1" (`self.DesiredLevel`)))
      (`/Game/Blueprints/UI/Gameplay/WBP_ScoreLevelsOnMap.SetScores` _aswbp_score_levels_on_map _bestscore _scorelevels))
    (:`Is Not Valid`
      _))
  (`/Game/Blueprints/Systems/Interaction/BPC_Interaction.ShowPrompt` (`self.BPC_Interaction`)))

(event `/Game/Blueprints/Systems/Interaction/BPI_Interaction.OnInteract`
  (params (Actor :type "Actor Object Reference"))
  (`/Game/Blueprints/Systems/Interaction/BPC_Interaction.Interact` (`self.BPC_Interaction`) true))

(event `self.BPC_Interaction.OnInteract`
  (params (CanInteract :type Boolean))
  (if CanInteract
    (bind _returnvalue (`|CreateWidget` "/Game/Blueprints/UI/Intro/WBP_LineDeathScreen.WBP_LineDeathScreen_C"))
    (`UserWidget.AddToViewport` _returnvalue 0)
    (bind _returnvalue_2 (`WorldPartitionBlueprintLibrary.GetDataLayerManager`))
    (`DataLayerManager.SetDataLayerRuntimeState` _returnvalue_2 (select `/Game/Blueprints/Systems/E_GameplayLevel` (`self.CurrentLevel`) :`NewEnumerator0` "/Game/Assets/DataLayers/LineModeLevel01.LineModeLevel01" :`NewEnumerator1` "/Game/Assets/DataLayers/LineModeLevel02.LineModeLevel02" :!type "DataLayerAsset Object Reference") "Unloaded" false)
    (`DataLayerManager.SetDataLayerRuntimeState` _returnvalue_2 (select `/Game/Blueprints/Systems/E_GameplayLevel` (`self.DesiredLevel`) :`NewEnumerator0` "/Game/Assets/DataLayers/LineModeLevel01.LineModeLevel01" :`NewEnumerator1` "/Game/Assets/DataLayers/LineModeLevel02.LineModeLevel02" :!type "DataLayerAsset Object Reference") "Activated" false)
    (`KismetSystemLibrary.Delay` 1.0)
    (bind _returnvalue_3 (`GameplayStatics.GetActorOfClass` "/Game/Blueprints/Systems/LineMode/Dream/BP_LineModeStarter.BP_LineModeStarter_C"))
    (`/Engine/EditorBlueprintResources/StandardMacros.IsValid` _returnvalue_3
      (:`Is Valid`
        (set `/Game/Blueprints/Systems/LineMode/Dream/BP_LineModeStarter.bStarted` false _returnvalue_3)
        (`self.K2_SetActorLocation` (`GameplayStatics.GetPlayerCharacter` 0) (`self.K2_GetActorLocation` _returnvalue_3) false false)))))

(fn `UserConstructionScript`)