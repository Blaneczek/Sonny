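; Grid tile for the Dream line mode path puzzle, where the player traces a line from first to final block without revisiting tiles.
; Highlighting marks the previous block and makes only unmarked neighbors, found by editor-time box overlaps, available.
; Dead ends update score, flicker the path and reset; the final block broadcasts completion through interfaces and unblocks BP_LineModeEnd.
; Side collision boxes touching adjacent blocks are disabled, and disabled blocks can be re-enabled.
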(event `self.ReceiveBeginPlay`
  (set `self.bMarked` false)
  (if (`self.bFirstBlock`)
    (set `self.bAvailable` true)
    (`KismetArrayLibrary.Array_Add` (`self.Tags`) "first")))

(event `/Game/Blueprints/Systems/LineMode/BPI_Lines.HighlightBlock`
  (params (PreviousBlock :type "Actor Object Reference"))
  (if (`self.bAvailable`)
    (if (not (`self.bFirstBlock`))
      (message `/Game/Blueprints/Systems/LineMode/BPI_Lines.MarkBlock` PreviousBlock))
    (`PrimitiveComponent.SetMaterial` (`self.Cube`) 0 "/Engine/MapTemplates/Materials/BasicAsset03.BasicAsset03")
    (if (`self.bFinalBlock`)
      ;[0.006655 0.05899 0.15 0.5] LineModeFinished
      (message `/Game/Blueprints/Characters/NPC/IntroReality/BPI_IntroRealityNPC.FinishLineGameplay` (`GameplayStatics.GetPlayerCharacter` 0))
      (bind _outactors (`GameplayStatics.GetAllActorsWithInterface` "/Game/Blueprints/Systems/LineMode/BPI_Lines.BPI_Lines_C"))
      (for _array_element _outactors
        (message `/Game/Blueprints/Systems/LineMode/BPI_Lines.PathFinished` _array_element))
      (bind _returnvalue (`GameplayStatics.GetActorOfClass` "/Game/Blueprints/Systems/LineMode/Dream/BP_LineModeEnd.BP_LineModeEnd_C"))
      (`/Engine/EditorBlueprintResources/StandardMacros.IsValid` _returnvalue
        (:`Is Valid`
          (`/Game/Blueprints/Systems/LineMode/Dream/BP_LineModeEnd.UnblockEnd` _returnvalue)))
      (else
        (message `/Game/Blueprints/Systems/LineMode/BPI_Lines.BlockPreviousPaths` PreviousBlock)
        (for _array_element_2 (`self.NeighborBlocks`)
          (bind _ismarked (message `/Game/Blueprints/Systems/LineMode/BPI_Lines.GetMarked` _array_element_2))
          (if (not _ismarked)
            (message `/Game/Blueprints/Systems/LineMode/BPI_Lines.SetAvailable` _array_element_2 true)
            (`/Engine/EditorBlueprintResources/StandardMacros.IncrementInt` (`self.counter`))))
        (if (> (`self.counter`) 0)
          (set `self.counter` 0)
          (else
            (set `self.counter` 0)
            (`KismetSystemLibrary.Delay` 0.5)
            ;[0.15 0.02519 0.07925 0.5] Bad Path
            (message `/Game/Blueprints/GameModes/Dreams/BPI_DreamGameMode.UpdateLineModeScore` (`GameplayStatics.GetGameMode`) "NewEnumerator3")
            (bind _outactors_2 (`GameplayStatics.GetAllActorsWithInterface` "/Game/Blueprints/Systems/LineMode/Dream/BPI_LineModeDream.BPI_LineModeDream_C"))
            (for _array_element_3 _outactors_2
              (message `/Game/Blueprints/Systems/LineMode/Dream/BPI_LineModeDream.StopLineMode` _array_element_3))
            (bind _outactors_3 (`GameplayStatics.GetAllActorsWithInterface` "/Game/Blueprints/Systems/LineMode/BPI_Lines.BPI_Lines_C"))
            (for _array_element_4 _outactors_3
              (message `/Game/Blueprints/Systems/LineMode/BPI_Lines.BadPath` _array_element_4))
            (`KismetSystemLibrary.Delay` 1.5)
            (bind _outactors_4 (`GameplayStatics.GetAllActorsWithInterface` "/Game/Blueprints/Systems/LineMode/Dream/BPI_LineModeDream.BPI_LineModeDream_C"))
            (for _array_element_5 _outactors_4
              (message `/Game/Blueprints/Systems/LineMode/Dream/BPI_LineModeDream.ResetLineMode` _array_element_5))))))))

(event `/Game/Blueprints/Systems/LineMode/BPI_Lines.BlockPreviousPaths`
  (for _array_element (`self.NeighborBlocks`)
    (message `/Game/Blueprints/Systems/LineMode/BPI_Lines.SetAvailable` _array_element false)))

(event `GetNeighborBlocks`
  ;[0.1464 0.0341 0.15 0.5] Setup in editor
  (`KismetArrayLibrary.Array_Clear` (`self.NeighborBlocks`))
  (`BlueprintSetLibrary.Set_Clear` (`self.tempSet`))
  (bind _outactors (`KismetSystemLibrary.BoxOverlapActors` (`self.K2_GetActorLocation`) (`KismetMathLibrary.Vector_GetAbs` (* 100.0 (`self.GetActorForwardVector`))) (`|MakeArray` "ObjectTypeQuery5" :!type "EObjectTypeQuery Enum") "BP_LineBlockDream_C" (`|MakeArray` self :!type "Actor Object Reference")))
  (`BlueprintSetLibrary.Set_AddItems` (`self.tempSet`) _outactors)
  (bind _outactors_2 (`KismetSystemLibrary.BoxOverlapActors` (`self.K2_GetActorLocation`) (`KismetMathLibrary.Vector_GetAbs` (* 100.0 (`self.GetActorRightVector`))) (`|MakeArray` "ObjectTypeQuery5" :!type "EObjectTypeQuery Enum") "BP_LineBlockDream_C" (`|MakeArray` self :!type "Actor Object Reference")))
  (`BlueprintSetLibrary.Set_AddItems` (`self.tempSet`) _outactors_2)
  (bind _result (`BlueprintSetLibrary.Set_ToArray` (`self.tempSet`)))
  (set `self.NeighborBlocks` _result)
  ;;[0 0.01513 0.15 0.5] Initialize first block
  (if (`self.bFirstBlock`)
    (`self.InitializeFirstBlock`)))

(event `/Game/Blueprints/Systems/LineMode/BPI_Lines.Reset`
  (set `self.bMarked` false)
  (if (`self.bFirstBlock`)
    (set `self.bAvailable` true)
    (`PrimitiveComponent.SetMaterial` (`self.Cube`) 0 "/Engine/MapTemplates/Materials/BasicAsset03.BasicAsset03")
    (`KismetSystemLibrary.Delay` 0.5)
    (`self.InitializeFirstBlock`)
    (else
      (set `self.bAvailable` false)
      (`PrimitiveComponent.SetMaterial` (`self.Cube`) 0 "/Engine/BasicShapes/BasicShapeMaterial.BasicShapeMaterial"))))

(event `/Game/Blueprints/Systems/LineMode/BPI_Lines.SetAvailable`
  (params (IsAvailable :type Boolean))
  (set `self.bAvailable` IsAvailable))

(event `/Game/Blueprints/Systems/LineMode/BPI_Lines.BadPath`
  (if (`self.bMarked`)
    (bind _returnvalue (`KismetSystemLibrary.K2_SetTimerDelegate` (delegate `Flicker`) 0.2 true))
    (set `self.FlickerTimer` _returnvalue)
    (`KismetSystemLibrary.Delay` 2.0)
    (`KismetSystemLibrary.K2_ClearAndInvalidateTimerHandle` (`self.FlickerTimer`))
    (`self.Reset`)))

(event `Flicker`
  (`/Engine/EditorBlueprintResources/StandardMacros.FlipFlop`
    (:`A`
      (`PrimitiveComponent.SetMaterial` (`self.Cube`) 0 "/Engine/MapTemplates/Materials/BasicAsset01.BasicAsset01"))
    (:`B`
      (`PrimitiveComponent.SetMaterial` (`self.Cube`) 0 "/Engine/MapTemplates/Materials/BasicAsset02.BasicAsset02"))))

(event `/Game/Blueprints/Systems/LineMode/BPI_Lines.PathFinished`
  (if (`self.bMarked`)
    (`PrimitiveComponent.SetMaterial` (`self.Cube`) 0 "/Engine/MapTemplates/Materials/BasicAsset03.BasicAsset03")))

(event `/Game/Blueprints/Systems/LineMode/BPI_Lines.RemoveOverlappingBoxes `
  (`self.RemoveOverlappingBoxes`))

(event `/Game/Blueprints/Systems/LineMode/BPI_Lines.ResetColors`
  (if (`self.bDisabled`)
    (`self.DisableBlock`)
    (else
      (`PrimitiveComponent.SetMaterial` (`self.Cube`) 0 "/Engine/BasicShapes/BasicShapeMaterial.BasicShapeMaterial"))))

(event `/Game/Blueprints/Systems/LineMode/BPI_Lines.SetEnableBlock`
  (`self.EnableBlock`))

(fn `DisableBlock`
  (`PrimitiveComponent.SetMaterial` (`self.Cube`) 0 "/Game/Assets/Materials/Dream/M_DisabledLMBlock.M_DisabledLMBlock"))

(fn `EnableBlock`
  (`PrimitiveComponent.SetMaterial` (`self.Cube`) 0 "/Engine/BasicShapes/BasicShapeMaterial.BasicShapeMaterial")
  (set `self.bDisabled` false)
  (`self.RemoveOverlappingBoxes`))

(fn `GetMarked`
  (returns (IsMarked :type Boolean))
  (return (`self.bMarked`)))

(fn `InitializeFirstBlock`
  (`self.HighlightBlock` null)
  (message `/Game/Blueprints/Systems/LineMode/Dream/BPI_LineModeDream.SetFirstBlockRef` (`GameplayStatics.GetPlayerCharacter` 0) self))

(fn `IsAvailable`
  (returns (Available :type Boolean))
  (return (`self.bAvailable`)))

(fn `IsDisabled`
  (returns (Disabled :type Boolean))
  (return (`self.bDisabled`)))

(fn `MarkBlock`
  (`PrimitiveComponent.SetMaterial` (`self.Cube`) 0 "/Engine/MapTemplates/Materials/BasicAsset01.BasicAsset01")
  (set `self.bAvailable` false)
  (set `self.bMarked` true)
  (message `/Game/Blueprints/GameModes/Dreams/BPI_DreamGameMode.UpdateLineModeScore` (`GameplayStatics.GetGameMode`) "NewEnumerator0"))

(fn `RemoveOverlappingBoxes`
  (locals (tempBox :type "BoxComponent Object Reference"))
  (if (not (`self.bDisabled`))
    (`|ExecutionSequence`
      (:`then_0`
        (set `local.tempBox` (`self.BoxLeft`))
        (if (`KismetArrayLibrary.Array_IsNotEmpty` (`PrimitiveComponent.GetOverlappingActors` (`local.tempBox`) "BP_LineBlockDream_C")) :!label _label
          (`PrimitiveComponent.SetCollisionEnabled` (`local.tempBox`) "NoCollision")))
      (:`then_1`
        (set `local.tempBox` (`self.BoxRight`))
        (goto _label))
      (:`then_2`
        (set `local.tempBox` (`self.BoxForward`))
        (goto _label))
      (:`then_3`
        (set `local.tempBox` (`self.BoxBack`))
        (goto _label))
      (:`then_4`
        (if (or (`self.bFirstBlock`) (`self.bFinalBlock`))
          (`|ExecutionSequence`
            (:`then_0`
              (set `local.tempBox` (`self.BoxForward`)))
            (:`then_1`
              (set `local.tempBox` (`self.BoxBack`))))
          (`PrimitiveComponent.SetCollisionEnabled` (`local.tempBox`) "NoCollision"))))))

(fn `UserConstructionScript`)