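; BP_LineModeObject is a Line Mode pickup whose Type decides its effect when the player overlaps its sphere.
; Wall Destructor calls DestroyWallBlock on every BP_LineModeWall in the level, then destroys the pickup.
; Invisibility Charge queries the player through message calls, then grants a charge and is consumed only if the player is visible and the next charge index is below the number of uses.
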(event `self.Sphere1.OnComponentBeginOverlap`
  (params (OverlappedComponent :type "PrimitiveComponent Object Reference") (OtherActor :type "Actor Object Reference") (OtherComp :type "PrimitiveComponent Object Reference") (OtherBodyIndex :type Integer) (bFromSweep :type Boolean) (SweepResult :type "HitResult Structure (by ref)"))
  (bind _returnvalue (`GameplayStatics.GetPlayerCharacter` 0))
  (if (== OtherActor (`GameplayStatics.GetPlayerCharacter` 0))
    (switch `/Game/Blueprints/Systems/LineMode/Dream/E_LineModeObjectType` (`self.Type`)
      (:`NewEnumerator0`
        (`self.DestroyWall`)
        (`self.K2_DestroyActor`))
      (:`NewEnumerator1`
        (bind _invisible (message `/Game/Blueprints/Systems/LineMode/Dream/BPI_LineModeDream.IsInvisible` _returnvalue))
        (if (not _invisible)
          (bind _uses (message `/Game/Blueprints/Systems/LineMode/Dream/BPI_LineModeDream.GetNumberOfInvisibilityUses` _returnvalue))
          (bind _index (message `/Game/Blueprints/Systems/LineMode/Dream/BPI_LineModeDream.GetInvisibilityCurrentIndex` _returnvalue))
          (if (< (+ _index 1) _uses)
            (message `/Game/Blueprints/Systems/LineMode/Dream/BPI_LineModeDream.AddInvisibilityCharge` (`GameplayStatics.GetPlayerCharacter` 0))
            (`self.K2_DestroyActor`)))))))

(fn `DestroyWall`
  (bind _outactors (`GameplayStatics.GetAllActorsOfClass` "/Game/Blueprints/Systems/LineMode/Dream/BP_LineModeWall.BP_LineModeWall_C"))
  (for _array_element _outactors
    (`/Engine/EditorBlueprintResources/StandardMacros.IsValid` _array_element
      (:`Is Valid`
        (`/Game/Blueprints/Systems/LineMode/Dream/BP_LineModeWall.DestroyWallBlock` _array_element)))))

(fn `UserConstructionScript`)