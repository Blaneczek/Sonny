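; BP_LineBlock is one cell in the intro's line-drawing puzzle, where the player traces a path block by block.
; Highlighting an available block marks the previous one, closes its branches and opens unmarked neighbours, which an editor-run box overlap caches.
; Dead ends flicker marked blocks then reset all through BPI_Lines, while the final block notifies player, door and supervisor and ends the sequence.
; A DoOnce limits highlighting until reset.
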(event `self.ReceiveBeginPlay`
  (if (`self.bFirst`)
    (set `self.bAvailable` true)
    (`KismetArrayLibrary.Array_Add` (`self.Tags`) "first")))

(event `/Game/Blueprints/Systems/LineMode/BPI_Lines.StartFirstFlickering`
  (if (`self.bFirst`)
    (bind _returnvalue (`KismetSystemLibrary.K2_SetTimerDelegate` (delegate `Flickering`) 0.2 true))
    (set `self.StartingFlickerTimer` _returnvalue)))

(event `Flickering`
  (bind _cube (`self.Cube`))
  (`/Engine/EditorBlueprintResources/StandardMacros.FlipFlop`
    (:`A`
      (`PrimitiveComponent.SetMaterial` _cube 0 "/Engine/MapTemplates/Materials/BasicAsset03.BasicAsset03"))
    (:`B`
      (`PrimitiveComponent.SetMaterial` _cube 0 "/Engine/BasicShapes/BasicShapeMaterial.BasicShapeMaterial"))))

(event `ResetDoOnce`
  (goto _label :!via `Reset`))

(event `/Game/Blueprints/Systems/LineMode/BPI_Lines.HighlightBlock`
  (params (PreviousBlock :type "Actor Object Reference"))
  (`KismetSystemLibrary.K2_ClearAndInvalidateTimerHandle` (`self.StartingFlickerTimer`))
  (if (`self.bAvailable`)
    (`/Engine/EditorBlueprintResources/StandardMacros.DoOnce` false :!label _label
      (:`Completed`
        (if (not (`self.bFirst`))
          (message `/Game/Blueprints/Systems/LineMode/BPI_Lines.MarkBlock` PreviousBlock))
        (`PrimitiveComponent.SetMaterial` (`self.Cube`) 0 "/Engine/MapTemplates/Materials/BasicAsset03.BasicAsset03")
        (if (`self.bFinalBlock`)
          (message `/Game/Blueprints/Characters/NPC/IntroReality/BPI_IntroRealityNPC.FinishLineGameplay` (`GameplayStatics.GetPlayerCharacter` 0))
          (bind _returnvalue (`GameplayStatics.GetActorOfClass` "/Game/Blueprints/Systems/LineMode/BP_Door.BP_Door_C"))
          (`/Game/Blueprints/Systems/LineMode/BP_Door.TurnGreen` _returnvalue)
          (bind _outactors (`GameplayStatics.GetAllActorsWithInterface` "/Game/Blueprints/Systems/LineMode/BPI_Lines.BPI_Lines_C"))
          (for _array_element _outactors
            (message `/Game/Blueprints/Systems/LineMode/BPI_Lines.PathFinished` _array_element))
          (bind _returnvalue_2 (`GameplayStatics.GetActorOfClass` "/Game/Blueprints/Characters/NPC/IntroReality/BP_IntroSupervisor.BP_IntroSupervisor_C"))
          (message `/Game/Blueprints/Characters/NPC/IntroReality/BPI_IntroRealityNPC.FinishLineGameplay` _returnvalue_2)
          (else
            (message `/Game/Blueprints/Systems/LineMode/BPI_Lines.BlockPreviousPaths` PreviousBlock)
            (for _array_element_2 (`self.NeighborBlocks`)
              (bind _ismarked (message `/Game/Blueprints/Systems/LineMode/BPI_Lines.GetMarked` _array_element_2))
              (if (not _ismarked)
                (message `/Game/Blueprints/Systems/LineMode/BPI_Lines.SetAvailable` _array_element_2 true)
                (`/Engine/EditorBlueprintResources/StandardMacros.IncrementInt` (`self.counter`))))
            (if (> (`self.counter`) 0)
              (set `self.counter` 0)
              (else
                (set `self.counter` 0)
                (message `/Game/Blueprints/Characters/NPC/IntroReality/BPI_IntroRealityNPC.NullBlock` (`GameplayStatics.GetPlayerCharacter` 0))
                (bind _outactors_2 (`GameplayStatics.GetAllActorsWithInterface` "/Game/Blueprints/Systems/LineMode/BPI_Lines.BPI_Lines_C"))
                (for _array_element_3 _outactors_2
                  (message `/Game/Blueprints/Systems/LineMode/BPI_Lines.BadPath` _array_element_3))
                (`KismetSystemLibrary.Delay` 2.2)
                (bind _outactors_3 (`GameplayStatics.GetAllActorsWithInterface` "/Game/Blueprints/Systems/LineMode/BPI_Lines.BPI_Lines_C"))
                (for _array_element_4 _outactors_3
                  (message `/Game/Blueprints/Systems/LineMode/BPI_Lines.Reset` _array_element_4))
                (message `/Game/Blueprints/Characters/NPC/IntroReality/BPI_IntroRealityNPC.SetLineMode` (`GameplayStatics.GetPlayerCharacter` 0) true)))))))))

(event `/Game/Blueprints/Systems/LineMode/BPI_Lines.BlockPreviousPaths`
  (for _array_element (`self.NeighborBlocks`)
    (message `/Game/Blueprints/Systems/LineMode/BPI_Lines.SetAvailable` _array_element false)))

(event `GetNeighborBlocks`
  ;[0.1464 0.0341 0.15 0.5] Setup in editor
  (`KismetArrayLibrary.Array_Clear` (`self.NeighborBlocks`))
  (`BlueprintSetLibrary.Set_Clear` (`self.tempSet`))
  (bind _outactors (`KismetSystemLibrary.BoxOverlapActors` (`self.K2_GetActorLocation`) (`KismetMathLibrary.Vector_GetAbs` (* 25.0 (`self.GetActorForwardVector`))) (`|MakeArray` "ObjectTypeQuery5" :!type "EObjectTypeQuery Enum") "BP_LineBlock_C" (`|MakeArray` self :!type "Actor Object Reference")))
  (`BlueprintSetLibrary.Set_AddItems` (`self.tempSet`) _outactors)
  (bind _outactors_2 (`KismetSystemLibrary.BoxOverlapActors` (`self.K2_GetActorLocation`) (`KismetMathLibrary.Vector_GetAbs` (* 25.0 (`self.GetActorUpVector`))) (`|MakeArray` "ObjectTypeQuery5" :!type "EObjectTypeQuery Enum") "BP_LineBlock_C" (`|MakeArray` self :!type "Actor Object Reference")))
  (`BlueprintSetLibrary.Set_AddItems` (`self.tempSet`) _outactors_2)
  (bind _result (`BlueprintSetLibrary.Set_ToArray` (`self.tempSet`)))
  (set `self.NeighborBlocks` _result))

(event `/Game/Blueprints/Systems/LineMode/BPI_Lines.Reset`
  (`self.ResetDoOnce`)
  (set `self.bMarked` false)
  (if (`self.bFirst`)
    (set `self.bAvailable` true)
    (`PrimitiveComponent.SetMaterial` (`self.Cube`) 0 "/Engine/MapTemplates/Materials/BasicAsset03.BasicAsset03")
    (else
      (set `self.bAvailable` false)
      (`PrimitiveComponent.SetMaterial` (`self.Cube`) 0 "/Engine/BasicShapes/BasicShapeMaterial.BasicShapeMaterial"))))

(event `/Game/Blueprints/Systems/LineMode/BPI_Lines.SetAvailable`
  (params (IsAvailable :type Boolean))
  (set `self.bAvailable` IsAvailable))

(event `/Game/Blueprints/Systems/LineMode/BPI_Lines.BadPath`
  (if (`self.bMarked`)
    (bind _returnvalue (`KismetSystemLibrary.K2_SetTimerDelegate` (delegate `Flicker`) 0.2 true))
    (set `self.FlickerTimer` _returnvalue)
    (`KismetSystemLibrary.Delay` 2.0)
    (`KismetSystemLibrary.K2_ClearAndInvalidateTimerHandle` (`self.FlickerTimer`))))

(event `Flicker`
  (`/Engine/EditorBlueprintResources/StandardMacros.FlipFlop`
    (:`A`
      (`PrimitiveComponent.SetMaterial` (`self.Cube`) 0 "/Engine/MapTemplates/Materials/BasicAsset01.BasicAsset01"))
    (:`B`
      (`PrimitiveComponent.SetMaterial` (`self.Cube`) 0 "/Engine/MapTemplates/Materials/BasicAsset02.BasicAsset02"))))

(event `/Game/Blueprints/Systems/LineMode/BPI_Lines.PathFinished`
  (if (`self.bMarked`)
    (`PrimitiveComponent.SetMaterial` (`self.Cube`) 0 "/Engine/MapTemplates/Materials/BasicAsset03.BasicAsset03")
    (bind _asbp_intro_reality_game_mode (cast `/Game/Blueprints/GameModes/Reality/BP_IntroRealityGameMode` (`GameplayStatics.GetGameMode`)))
    (`/Game/Blueprints/GameModes/Reality/BP_IntroRealityGameMode.EndSequence1` _asbp_intro_reality_game_mode)))

(fn `GetMarked`
  (returns (IsMarked :type Boolean))
  (return (`self.bMarked`)))

(fn `IsAvailable`
  (returns (Available :type Boolean))
  (return (`self.bAvailable`)))

(fn `MarkBlock`
  (`PrimitiveComponent.SetMaterial` (`self.Cube`) 0 "/Engine/MapTemplates/Materials/BasicAsset01.BasicAsset01")
  (set `self.bAvailable` false)
  (set `self.bMarked` true))

(fn `UserConstructionScript`)