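; BP_StartingPlatform is a starting platform for the Line Mode system that switches between two collision setups.
; On BeginPlay it turns on query and physics collision for the BoxIn component.
; EnableCollision turns that collision on for five other box components and disables it on BoxIn.
; The Blueprint never calls EnableCollision itself and has no logic to reverse the switch.
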(event `self.ReceiveBeginPlay`
  (`PrimitiveComponent.SetCollisionEnabled` (`self.BoxIn`) "QueryAndPhysics"))

(fn `EnableCollision`
  (`PrimitiveComponent.SetCollisionEnabled` (`self.Box`) "QueryAndPhysics")
  (`PrimitiveComponent.SetCollisionEnabled` (`self.Box1`) "QueryAndPhysics")
  (`PrimitiveComponent.SetCollisionEnabled` (`self.Box2`) "QueryAndPhysics")
  (`PrimitiveComponent.SetCollisionEnabled` (`self.Box3`) "QueryAndPhysics")
  (`PrimitiveComponent.SetCollisionEnabled` (`self.Box4`) "QueryAndPhysics")
  (`PrimitiveComponent.SetCollisionEnabled` (`self.BoxIn`) "NoCollision"))

(fn `UserConstructionScript`)