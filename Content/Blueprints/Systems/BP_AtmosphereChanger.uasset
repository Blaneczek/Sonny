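; BP_AtmosphereChanger is a trigger volume that changes the sky atmosphere's look to match a chosen level.
; The first overlap of its Box by any actor passes a DoOnce and switches on the Level value, with the NONE case using the epilog albedo.
; Each case finds the SkyAtmosphere actor and sets its ground albedo from a per-level variable and its Rayleigh scattering to a hardcoded color.
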(event `self.Box.OnComponentBeginOverlap`
  (params (OverlappedComponent :type "PrimitiveComponent Object Reference") (OtherActor :type "Actor Object Reference") (OtherComp :type "PrimitiveComponent Object Reference") (OtherBodyIndex :type Integer) (bFromSweep :type Boolean) (SweepResult :type "HitResult Structure (by ref)"))
  (`/Engine/EditorBlueprintResources/StandardMacros.DoOnce` false
    (:`Completed`
      (switch `/Game/Blueprints/Systems/E_GameplayLevel` (`self.Level`)
        (:`NewEnumerator3`
          (bind _returnvalue (`GameplayStatics.GetActorOfClass` "/Script/Engine.SkyAtmosphere"))
          (`/Engine/EditorBlueprintResources/StandardMacros.IsValid` _returnvalue
            (:`Is Valid`
              (bind _skyatmospherecomponent (`SkyAtmosphere.SkyAtmosphereComponent` _returnvalue))
              (`SkyAtmosphereComponent.SetGroundAlbedo` _skyatmospherecomponent (`self.EpilogAlbedo`))
              (`SkyAtmosphereComponent.SetRayleighScattering` _skyatmospherecomponent (struct :`R` 0.25098 :`G` 0.623529 :`B` 0.870588 :`A` 1.0)))))
        (:`NewEnumerator0`
          (bind _returnvalue_2 (`GameplayStatics.GetActorOfClass` "/Script/Engine.SkyAtmosphere"))
          (`/Engine/EditorBlueprintResources/StandardMacros.IsValid` _returnvalue_2
            (:`Is Valid`
              (bind _skyatmospherecomponent_2 (`SkyAtmosphere.SkyAtmosphereComponent` _returnvalue_2))
              (`SkyAtmosphereComponent.SetGroundAlbedo` _skyatmospherecomponent_2 (`self.Level01Albedo`))
              (`SkyAtmosphereComponent.SetRayleighScattering` _skyatmospherecomponent_2 (struct :`R` 0.098039 :`G` 0.215686 :`B` 1.0 :`A` 1.0)))))
        (:`NewEnumerator1`
          (bind _returnvalue_3 (`GameplayStatics.GetActorOfClass` "/Script/Engine.SkyAtmosphere"))
          (`/Engine/EditorBlueprintResources/StandardMacros.IsValid` _returnvalue_3
            (:`Is Valid`
              (bind _skyatmospherecomponent_3 (`SkyAtmosphere.SkyAtmosphereComponent` _returnvalue_3))
              (`SkyAtmosphereComponent.SetGroundAlbedo` _skyatmospherecomponent_3 (`self.Level02Albedo`))
              (`SkyAtmosphereComponent.SetRayleighScattering` _skyatmospherecomponent_3 (struct :`R` 0.894118 :`G` 0.796079 :`B` 1.0 :`A` 1.0)))))
        (:`NewEnumerator2`
          (bind _returnvalue_4 (`GameplayStatics.GetActorOfClass` "/Script/Engine.SkyAtmosphere"))
          (`/Engine/EditorBlueprintResources/StandardMacros.IsValid` _returnvalue_4
            (:`Is Valid`
              (bind _skyatmospherecomponent_4 (`SkyAtmosphere.SkyAtmosphereComponent` _returnvalue_4))
              (`SkyAtmosphereComponent.SetGroundAlbedo` _skyatmospherecomponent_4 (`self.Level03Albedo`))
              (`SkyAtmosphereComponent.SetRayleighScattering` _skyatmospherecomponent_4 (struct :`R` 1.0 :`G` 0.635294 :`B` 0.592157 :`A` 1.0)))))))))

(fn `UserConstructionScript`)