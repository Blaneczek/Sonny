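; BPC_Dialogue is a dialogue component that puts a conversation on screen and signals when it ends.
; StartDialog casts its Dialogue reference to BP_DialogueDataBase, passes that data to a new WBP_Dialogue, and switches to UI-only input with the cursor hidden.
; It binds the widget's end event only when FirstTime is true.
; The DialogueEnd event rebroadcasts through the component's OnDialogueEnd dispatcher.
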(event `DialogueEnd`
  (`self.OnDialogueEnd`))

(fn `StartDialog`
  (params (bFirstTime :type Boolean))
  (bind _returnvalue (`GameplayStatics.GetPlayerController` 0))
  (bind _asbp_dialogue_data_base (cast `/Game/Blueprints/Systems/Dialogues/BP_DialogueDataBase` (`self.Dialogue`)))
  (`/Engine/EditorBlueprintResources/StandardMacros.IsValid` _asbp_dialogue_data_base
    (:`Is Valid`
      (bind _returnvalue_2 (`|CreateWidget` "/Game/Blueprints/UI/Narrative/WBP_Dialogue.WBP_Dialogue_C" null (`/Game/Blueprints/Systems/Dialogues/BP_DialogueDataBase.Dialogue` _asbp_dialogue_data_base)))
      (`UserWidget.AddToViewport` _returnvalue_2 0)
      (`WidgetBlueprintLibrary.SetInputMode_UIOnlyEx` _returnvalue _returnvalue_2)
      (set `PlayerController.bShowMouseCursor` false _returnvalue)
      (if bFirstTime
        (add `/Game/Blueprints/UI/Narrative/WBP_Dialogue.OnDialogueEnd` _returnvalue_2 (`|CreateDelegate` :!event `DialogueEnd`))))))