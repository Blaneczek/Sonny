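; Game mode for dream levels that runs scoring and progression for Line Mode and Combat gameplay, relaying updates to the HUD.
; Typed events and a looping clock adjust a clamped score; some Combat levels also periodically draw slow floors on combat floor actors.
; Level end pauses the game, awards upgrade points for newly reached thresholds and records best scores.
; Per-mode maps hold thresholds, bests and upgradeable stats.
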(event `/Game/Blueprints/GameModes/Dreams/BPI_DreamGameMode.StartAbility`
  (params (Index :type Integer))
  ;[0.01641 0.04432 0.15 0.5] Ability
  (bind _hudref (`self.HUDRef`)
    (:`then`
      (message `/Game/Blueprints/UI/HUD/BPI_DreamHUD.StartAbility` _hudref Index))
    (:`else`)))

(event `self.ReceiveBeginPlay`
  (`KismetSystemLibrary.Delay` 0.2)
  (set `self.HUDRef` (`PlayerController.GetHUD` (`GameplayStatics.GetPlayerController` 0))))

(event `/Game/Blueprints/GameModes/Dreams/BPI_DreamGameMode.RechargeAbility`
  (params (Index :type Integer) (bAllCharges :type Boolean))
  ;[0.01641 0.04432 0.15 0.5] Ability
  (bind _hudref (`self.HUDRef`)
    (:`then`
      (message `/Game/Blueprints/UI/HUD/BPI_DreamHUD.RechargeAbility` _hudref Index bAllCharges))
    (:`else`)))

(event `/Game/Blueprints/GameModes/Dreams/BPI_DreamGameMode.UpdateLineModeScore`
  (params (Type :type "/Game/Blueprints/Systems/LineMode/Dream/E_LineModeScoreModifier Enum" :default "NewEnumerator0"))
  ;[0.008996 0.15 0.04678 0.5] LineMode
  (switch `/Game/Blueprints/Systems/LineMode/Dream/E_LineModeScoreModifier` Type
    (:`NewEnumerator0`
      (bind _output_get (set `self.PenaltyValue` 1))
      (set `self.CurrentScore` (`KismetMathLibrary.Clamp` (- (`self.CurrentScore`) _output_get) 0 1000)))
    (:`NewEnumerator1`
      (bind _output_get_2 (set `self.PenaltyValue` 30))
      (set `self.CurrentScore` (`KismetMathLibrary.Clamp` (- (`self.CurrentScore`) _output_get_2) 0 1000)))
    (:`NewEnumerator2`
      (bind _output_get_3 (set `self.PenaltyValue` 10))
      (set `self.CurrentScore` (`KismetMathLibrary.Clamp` (- (`self.CurrentScore`) _output_get_3) 0 1000)))
    (:`NewEnumerator3`
      (bind _output_get_4 (set `self.PenaltyValue` 20))
      (set `self.CurrentScore` (`KismetMathLibrary.Clamp` (- (`self.CurrentScore`) _output_get_4) 0 1000))))
  (bind _hudref (`self.HUDRef`)
    (:`then`
      (message `/Game/Blueprints/UI/HUD/BPI_DreamHUD.UpdateLineModeScore` _hudref (`self.CurrentScore`) (`self.PenaltyValue`) Type))
    (:`else`)))

(event `/Game/Blueprints/GameModes/Dreams/BPI_DreamGameMode.StartGameplayLevel`
  (params (Level :type "/Game/Blueprints/Systems/E_GameplayLevel Enum" :default "NewEnumerator3") (GameplayType :type "/Game/Blueprints/Characters/Sonny/Dream/E_GameplayType Enum" :default "NewEnumerator0"))
  (`|ExecutionSequence`
    (:`then_0`
      (`self.SetGameplayVariables` Level GameplayType)
      (bind _hudref (`self.HUDRef`)
        (:`then`
          (message `/Game/Blueprints/UI/HUD/BPI_DreamHUD.StartGameplay` _hudref (`self.StartingScore`) (`self.GameplayType`) (`self.ScoreThresholds`))
          (bind _returnvalue (`KismetSystemLibrary.K2_SetTimerDelegate` (delegate `Clock`) 10.0 true))
          (set `self.ClockTimer` _returnvalue))
        (:`else`)))
    (:`then_1`
      (if (and (`|EnumEquality` GameplayType "NewEnumerator2") (or (`|EnumEquality` Level "NewEnumerator1") (`|EnumEquality` Level "NewEnumerator2")))
        (bind _returnvalue_2 (`KismetSystemLibrary.K2_SetTimerDelegate` (delegate `SpawnSlowFloor`) 30.0 true))
        (set `self.SlowFloorTimer` _returnvalue_2)))))

(event `Clock`
  (switch `/Game/Blueprints/Characters/Sonny/Dream/E_GameplayType` (`self.GameplayType`)
    (:`NewEnumerator1`
      (`self.UpdateLineModeScore` "NewEnumerator2"))
    (:`NewEnumerator2`
      (`self.UpdateCombatModeScore` "NewEnumerator0"))))

(event `/Game/Blueprints/GameModes/Dreams/BPI_DreamGameMode.UpgradeLineModeStats`
  (params (UpgradeType :type "/Game/Blueprints/Systems/LineMode/Dream/E_LineModeUpgradeType Enum" :default "NewEnumerator4") (Value :type "Float (double-precision)"))
  ;[0.008996 0.15 0.04678 0.5] LineMode
  (`BlueprintMapLibrary.Map_Add` (`self.LineModeStats`) UpgradeType (+ Value (`BlueprintMapLibrary.Map_Find` (`self.LineModeStats`) UpgradeType))))

(event `SpawnSlowFloor`
  (bind _outactors (`GameplayStatics.GetAllActorsOfClass` "/Game/Blueprints/Systems/Combat/BP_CombatFloor.BP_CombatFloor_C"))
  (for _array_element _outactors
    (message `/Game/Blueprints/Systems/Combat/BPI_CombatFloor.DrawSlowFloor` _array_element)))

(event `/Game/Blueprints/GameModes/Dreams/BPI_DreamGameMode.EndGameplayLevel`
  (`KismetSystemLibrary.Delay` 0.2)
  (`GameplayStatics.SetGamePaused` true)
  (`KismetSystemLibrary.K2_ClearAndInvalidateTimerHandle` (`self.ClockTimer`))
  (`KismetSystemLibrary.K2_ClearAndInvalidateTimerHandle` (`self.SlowFloorTimer`))
  (bind (_bnewscorelevel _upgradepoints) (`self.CheckScoreRewards`))
  (bind _lastbestscore (`self.CheckIfNewBestScore`))
  (bind _hudref (`self.HUDRef`)
    (:`then`
      (message `/Game/Blueprints/UI/HUD/BPI_DreamHUD.SetScoreLevels` _hudref (`self.ScoreThresholds`))
      (switch `/Game/Blueprints/Characters/Sonny/Dream/E_GameplayType` (`self.GameplayType`)
        (:`NewEnumerator1`
          (message `/Game/Blueprints/UI/HUD/BPI_DreamHUD.EndLineModeGameplay` _hudref _lastbestscore (`self.CurrentScore`) _bnewscorelevel _upgradepoints (`self.CurrentLevel`) (`BlueprintMapLibrary.Map_Find` (`self.LineModeUpgradeValues`) (`self.CurrentLevel`)) (`self.LineModeStats`)))
        (:`NewEnumerator2`
          (message `/Game/Blueprints/UI/HUD/BPI_DreamHUD.EndCombatGameplay` _hudref _lastbestscore (`self.CurrentScore`) _bnewscorelevel _upgradepoints (`self.CurrentLevel`) (`BlueprintMapLibrary.Map_Find` (`self.CombatUpgradeValues`) (`self.CurrentLevel`)) (`self.CombatStats`)))))
    (:`else`)))

(event `/Game/Blueprints/GameModes/Dreams/BPI_DreamGameMode.SetBlockNumber`
  (params (Number :type Integer))
  (bind _hudref (`self.HUDRef`)
    (:`then`
      (message `/Game/Blueprints/UI/HUD/BPI_DreamHUD.SetBlockNumber` _hudref Number))
    (:`else`)))

(event `/Game/Blueprints/GameModes/Dreams/BPI_DreamGameMode.UpdateCombatModeScore`
  (params (Type :type "/Game/Blueprints/Systems/Combat/E_CombatScoreModifier Enum" :default "NewEnumerator0"))
  ;[0.15 0.01505 0.04119 0.5] CombatMode
  (switch `/Game/Blueprints/Systems/Combat/E_CombatScoreModifier` Type
    (:`NewEnumerator0`
      (bind _output_get (set `self.PenaltyValue` 10))
      (set `self.CurrentScore` (`KismetMathLibrary.Clamp` (- (`self.CurrentScore`) _output_get) 0 1000)))
    (:`NewEnumerator4`
      (bind _output_get_2 (set `self.PenaltyValue` 40))
      (set `self.CurrentScore` (`KismetMathLibrary.Clamp` (- (`self.CurrentScore`) _output_get_2) 0 1000)))
    (:`NewEnumerator5`
      (bind _output_get_3 (set `self.PenaltyValue` 50))
      (set `self.CurrentScore` (`KismetMathLibrary.Clamp` (+ (`self.CurrentScore`) _output_get_3) 0 1000)))
    (:`NewEnumerator7`
      (bind _output_get_4 (set `self.PenaltyValue` 4))
      (set `self.CurrentScore` (`KismetMathLibrary.Clamp` (- (`self.CurrentScore`) _output_get_4) 0 1000))))
  (bind _hudref (`self.HUDRef`)
    (:`then`
      (message `/Game/Blueprints/UI/HUD/BPI_DreamHUD.UpdateCombatScore` _hudref (`self.CurrentScore`) (`self.PenaltyValue`) Type))
    (:`else`)))

(event `/Game/Blueprints/GameModes/Dreams/BPI_DreamGameMode.UpgradeCombatStats`
  (params (UpgradeType :type "/Game/Blueprints/Systems/Combat/E_CombatUpgradeType Enum" :default "NewEnumerator4") (Value :type "Float (double-precision)"))
  ;[0.15 0.01505 0.04119 0.5] CombatMode
  (`BlueprintMapLibrary.Map_Add` (`self.CombatStats`) UpgradeType (+ Value (`BlueprintMapLibrary.Map_Find` (`self.CombatStats`) UpgradeType))))

(fn `CheckIfNewBestScore`
  (returns (LastBestScore :type Integer))
  (locals (tempLastBestScore :type Integer))
  (bind _value (`BlueprintMapLibrary.Map_Find` (`self.LineModeBestScores`) (`self.CurrentLevel`)))
  (bind _value_2 (`BlueprintMapLibrary.Map_Find` (`self.CombatBestScores`) (`self.CurrentLevel`)))
  (switch `/Game/Blueprints/Characters/Sonny/Dream/E_GameplayType` (`self.GameplayType`)
    (:`NewEnumerator1`
      (set `local.tempLastBestScore` _value)
      (if (> (`self.CurrentScore`) _value)
        (`BlueprintMapLibrary.Map_Add` (`self.LineModeBestScores`) (`self.CurrentLevel`) (`self.CurrentScore`))
        (return (`local.tempLastBestScore`))
        (else
          (return (`local.tempLastBestScore`)))))
    (:`NewEnumerator2`
      (set `local.tempLastBestScore` _value_2)
      (if (> (`self.CurrentScore`) _value_2)
        (`BlueprintMapLibrary.Map_Add` (`self.CombatBestScores`) (`self.CurrentLevel`) (`self.CurrentScore`))
        (return (`local.tempLastBestScore`))
        (else
          (return (`local.tempLastBestScore`)))))))

(fn `CheckScoreRewards`
  (returns (bNewScoreLevel :type Boolean) (UpgradePoints :type Integer))
  (locals (tempUpgradePoints :type Integer) (tempScoreThresholds :type "/Game/Blueprints/Systems/S_ScoreThresholds Structure") (tempIsNewScoreLevel :type Boolean))
  (set `local.tempUpgradePoints` 0)
  (switch `/Game/Blueprints/Characters/Sonny/Dream/E_GameplayType` (`self.GameplayType`)
    (:`NewEnumerator1`
      (set `local.tempScoreThresholds` (`BlueprintMapLibrary.Map_Find` (`self.LineModeScoreLevels`) (`self.CurrentLevel`))))
    (:`NewEnumerator2`
      (set `local.tempScoreThresholds` (`BlueprintMapLibrary.Map_Find` (`self.CombatScoreLevels`) (`self.CurrentLevel`)))))
  (bind _values (`BlueprintMapLibrary.Map_Values` (`.ScoreLevel_4_C616E5374C15C9182E866D8136782091` (break `/Game/Blueprints/Systems/S_ScoreThresholds` (`local.tempScoreThresholds`)))))
  (for (_array_element _array_index) _values
    (bind (_min _bgained) (break `/Game/Blueprints/Systems/S_ScoreAttributes` _array_element))
    (if _bgained
      _
      (elif (>= (`self.CurrentScore`) _min)
        (`/Engine/EditorBlueprintResources/StandardMacros.IncrementInt` (`local.tempUpgradePoints`)
          (:`  `
            (`BlueprintMapLibrary.Map_Add` (`.ScoreLevel_4_C616E5374C15C9182E866D8136782091` (break `/Game/Blueprints/Systems/S_ScoreThresholds` (`local.tempScoreThresholds`))) (+ _array_index 1) (make `/Game/Blueprints/Systems/S_ScoreAttributes` _min true))
            (set `local.tempIsNewScoreLevel` true))))))
  (switch `/Game/Blueprints/Characters/Sonny/Dream/E_GameplayType` (`self.GameplayType`)
    (:`NewEnumerator1`
      (`BlueprintMapLibrary.Map_Add` (`self.LineModeScoreLevels`) (`self.CurrentLevel`) (`local.tempScoreThresholds`))
      (`KismetSystemLibrary.PrintString` "jjjjjj"))
    (:`NewEnumerator2`
      (`BlueprintMapLibrary.Map_Add` (`self.CombatScoreLevels`) (`self.CurrentLevel`) (`local.tempScoreThresholds`))))
  (return (`local.tempIsNewScoreLevel`) (`local.tempUpgradePoints`)))

(fn `GetCombatStats`
  (returns (Stats :type "Map of /Game/Blueprints/Systems/Combat/E_CombatUpgradeType Enum to Float (double-precision)"))
  (return (`self.CombatStats`)))

(fn `GetLineModeStats`
  (returns (Stats :type "Map of /Game/Blueprints/Systems/LineMode/Dream/E_LineModeUpgradeType Enum to Float (double-precision)"))
  (return (`self.LineModeStats`)))

(fn `GetScores`
  (params (GameplayType :type "/Game/Blueprints/Characters/Sonny/Dream/E_GameplayType Enum" :default "NewEnumerator0") (Level :type "/Game/Blueprints/Systems/E_GameplayLevel Enum" :default "NewEnumerator3"))
  (returns (BestScore :type Integer) (ScoreLevels :type "/Game/Blueprints/Systems/S_ScoreThresholds Structure"))
  (switch `/Game/Blueprints/Characters/Sonny/Dream/E_GameplayType` GameplayType
    (:`NewEnumerator1`
      (return (`BlueprintMapLibrary.Map_Find` (`self.LineModeBestScores`) Level) (`BlueprintMapLibrary.Map_Find` (`self.LineModeScoreLevels`) Level)))
    (:`NewEnumerator2`
      (return (`BlueprintMapLibrary.Map_Find` (`self.CombatBestScores`) Level) (`BlueprintMapLibrary.Map_Find` (`self.CombatScoreLevels`) Level)))))

(fn `SetGameplayVariables`
  (params (Level :type "/Game/Blueprints/Systems/E_GameplayLevel Enum" :default "NewEnumerator3") (GameplayType :type "/Game/Blueprints/Characters/Sonny/Dream/E_GameplayType Enum" :default "NewEnumerator0"))
  (set `self.CurrentLevel` Level)
  (set `self.GameplayType` GameplayType)
  (set `self.Time` 0)
  (set `self.CurrentScore` (`self.StartingScore`))
  (switch `/Game/Blueprints/Characters/Sonny/Dream/E_GameplayType` (`self.GameplayType`)
    (:`NewEnumerator0`
      _)
    (:`NewEnumerator1`
      (set `self.ScoreThresholds` (`BlueprintMapLibrary.Map_Find` (`self.LineModeScoreLevels`) (`self.CurrentLevel`))))
    (:`NewEnumerator2`
      (set `self.ScoreThresholds` (`BlueprintMapLibrary.Map_Find` (`self.CombatScoreLevels`) (`self.CurrentLevel`)))))
  (return))

(fn `UserConstructionScript`)