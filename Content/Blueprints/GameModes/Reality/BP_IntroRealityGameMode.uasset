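; Game mode for the intro "Reality" level, which scripts the opening cinematic sequence around Sonny.
; On BeginPlay it creates the HUD, fades in, shows timed thought lines and tells BP_IntroRealitySonny to open a gate.
; EndSequence1 hides HUD pointer and controls, then between fades moves Sonny to a spawn point with an idle pose and end camera.
; A CameraFade helper drives transitions, and EndSequence2 opens Dream01Map.
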(event `self.ReceiveBeginPlay`
  (`KismetSystemLibrary.ExecuteConsoleCommand` "disableallscreenmessages" null)
  (bind _returnvalue (`|CreateWidget` "/Game/Blueprints/UI/HUD/WBP_IntroRealityHUD.WBP_IntroRealityHUD_C"))
  (bind _output_get (set `self.WidgetRef` _returnvalue))
  (`UserWidget.AddToViewport` _output_get 0)
  (`self.CameraFade` true 5.0)
  (`KismetSystemLibrary.Delay` 2.0)
  (`/Game/Blueprints/UI/HUD/WBP_IntroRealityHUD.ShowThought` (`self.WidgetRef`) 7.0 "What...? What... is going on...? Where... I... am...?")
  (`KismetSystemLibrary.Delay` (`.Scene1_2_54D202CD48CC0C362551958849B408F3` (break `/Game/Blueprints/GameModes/Reality/S_IntroRealityDelays` (`self.DelayTimes`))))
  (bind _returnvalue_2 (`GameplayStatics.GetActorOfClass` "/Game/Blueprints/Characters/Sonny/IntroReality/BP_IntroRealitySonny.BP_IntroRealitySonny_C"))
  (bind _output_get_2 (set `self.SonnyRef` _returnvalue_2))
  (`/Game/Blueprints/Characters/Sonny/IntroReality/BP_IntroRealitySonny.OpenGate` _output_get_2)
  (`KismetSystemLibrary.Delay` 3.0)
  (`/Game/Blueprints/UI/HUD/WBP_IntroRealityHUD.ShowThought` (`self.WidgetRef`) 5.0 "My body.... aghh... It moves by itself..."))

(event `EndSequence1`
  (bind _widgetref (`self.WidgetRef`))
  (`/Game/Blueprints/UI/HUD/WBP_IntroRealityHUD.SetPointerVisibility` _widgetref false)
  (`/Game/Blueprints/UI/HUD/WBP_IntroRealityHUD.SetControlsVisibility` _widgetref false)
  (`/Game/Blueprints/UI/HUD/WBP_IntroRealityHUD.ShowThought` (`self.WidgetRef`) 5.0 "It worked...!")
  (`KismetSystemLibrary.Delay` (`.Scene3_6_932027F548922B9AB00BECACFEBDAB86` (break `/Game/Blueprints/GameModes/Reality/S_IntroRealityDelays` (`self.DelayTimes`))))
  (`self.CameraFade` false 3.0)
  (`KismetSystemLibrary.Delay` 4.0)
  (`self.CameraFade` true 3.0)
  (bind _sonnyref (`self.SonnyRef`)
    (:`then`
      (bind _mesh (`Character.Mesh` _sonnyref))
      (`SkeletalMeshComponent.SetAnimationMode` _mesh "AnimationSingleNode" true)
      (`SkeletalMeshComponent.PlayAnimation` _mesh "/Game/Characters/Mannequins/Animations/Manny/MM_Idle.MM_Idle" false)
      (`/Game/Blueprints/Characters/Sonny/IntroReality/BP_IntroRealitySonny.SetEndCamera` _sonnyref)
      (bind _returnvalue (`GameplayStatics.GetActorOfClass` "/Game/Blueprints/Characters/Sonny/IntroReality/BP_SpawnPoint.BP_SpawnPoint_C"))
      (`self.K2_SetActorTransform` _sonnyref (`self.GetTransform` _returnvalue) false false)
      (`KismetSystemLibrary.Delay` 3.0)
      (`/Game/Blueprints/UI/HUD/WBP_IntroRealityHUD.ShowThought` (`self.WidgetRef`) 4.0 "Tomorrow.... my only... chance...")
      (`KismetSystemLibrary.Delay` 4.0)
      (`self.CameraFade` false 3.0)
      (`KismetSystemLibrary.Delay` 5.0)
      (`self.EndSequence2`))
    (:`else`)))

(event `EndSequence2`
  (`GameplayStatics.OpenLevelBySoftObjectPtr` "/Game/Maps/Dreams/Dream01Map.Dream01Map"))

(fn `CameraFade`
  (params (In :type Boolean) (Time :type "Float (double-precision)"))
  (bind _playercameramanager (`PlayerController.PlayerCameraManager` (`GameplayStatics.GetPlayerController` 0)))
  (if In
    (`PlayerCameraManager.StartCameraFade` :`self` _playercameramanager :`FromAlpha` 1.0 :`Duration` Time :`bHoldWhenFinished` true)
    (else
      (`PlayerCameraManager.StartCameraFade` :`self` _playercameramanager :`ToAlpha` 1.0 :`Duration` Time :`bHoldWhenFinished` true)))
  (return))

(fn `UserConstructionScript`)